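; Spline movement Blueprint that drives a referenced Cart along a spline while the cart's IsDriving flag is set.
; Construction places the cart at the first spline point, and BeginPlay sets the timeline play rate to 1/TimelineLength.
; Tick starts the timeline, whose alpha lerps distance along the spline to set cart location, local Y offset and tangent-aligned rotation.
; The timeline stops when IsDriving turns false, and clears that flag on finishing.
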(event Custom|Drive%20on%20Spline
  (bind _spline (Variables|Default|GetSpline))
  (bind _spline_2 (Variables|Default|GetSpline))
  (bind _cart (Variables|Default|Getcart))
  (bind _cart_2 (Variables|Default|Getcart))
  ;[0.4 0.95 0.3] Move cart along spline
  (bind _newtrack_0 (Timeline|Timeline Play)
    (:Update
      (if (== (Variables|/Game/Ouroboros/Core/BP_Cart.BP_Cart_C|GetisDriving _cart_2) true)
        ;;[1 1 1] set cart location on update
        (Transformation|SetActorLocation (Variables|Default|Getcart) (Spline|GetLocationatDistanceAlongSpline _spline_2 (Math|Float|Lerp 0.0 (Spline|GetDistanceAlongSplineatSplinePoint _spline (- (Spline|GetNumberOfSplinePoints _spline) 1)) _newtrack_0) "World") false false)
        (Transformation|AddActorLocalOffset _cart (Math|Vector|MakeVector 0.0 (Variables|/Game/Ouroboros/Core/BP_Cart.BP_Cart_C|Getoffset _cart) 0.0) false false)
        ;;[1 1 1] set cart rotation on update
        (Transformation|SetActorRotation _cart (Math|Conversions|RotationFromXVector (Spline|GetTangentatDistanceAlongSpline _spline_2 (Math|Float|Lerp 0.0 (Spline|GetDistanceAlongSplineatSplinePoint _spline (- (Spline|GetNumberOfSplinePoints _spline) 1)) _newtrack_0) "World")))
        (Variables|Default|SetsplineLength (Math|Float|Lerp 0.0 (Spline|GetDistanceAlongSplineatSplinePoint _spline (- (Spline|GetNumberOfSplinePoints _spline) 1)) _newtrack_0))
        (else
          (Timeline|Timeline Stop))))
    (:Finished
      (Variables|/Game/Ouroboros/Core/BP_Cart.BP_Cart_C|SetisDriving _cart_2 false))))

(event EventBeginPlay
  ;[0.4 0.95 0.3] Move cart along spline
  ;;[1 1 1] Set play rate on begin play
  ;;;[1 1 1 1 12] The Play Rate of a timeline indicates the speed at which the timeline is played.
  (Components|Timeline|SetPlayRate (Variables|Default|GetTimeline) (/ 1.0 (Variables|Default|GettimelineLength))))

(event EventTick
  (params (DeltaSeconds :type Float%20%28single-precision%29))
  ;[1 1 1] Trigger driving event
  (if (Variables|/Game/Ouroboros/Core/BP_Cart.BP_Cart_C|GetisDriving (Variables|Default|Getcart))
    (CallFunction|DriveonSpline)))

(fn ConstructionScript
  ;[1 1 1] set cart start point to point on spline with index zero on construction
  (Transformation|SetActorLocation (Variables|Default|Getcart) (Spline|GetLocationatSplinePoint (Variables|Default|GetSpline) 0 "World") false false))