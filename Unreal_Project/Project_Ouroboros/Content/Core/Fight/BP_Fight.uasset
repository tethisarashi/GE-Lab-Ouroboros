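; BP_Fight runs a turn-based battle between the GameInstance party and one to four spawned bandits, with a random starting side.
; Player actions and targets queue in a map through the fight and enemy widgets, then execute on confirm.
; Enemies act by chance-based heal, special or base attack, with special attacks limited by weapon round cooldowns.
; Sides alternate until one is wiped out, then it restores cart mode and destroys itself.
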(event Custom|Begin%20Next%20Round
  (if (== (Variables|Default|GetisPartiesTurn) true)
    ;[1 0 0] DEBUG
    (Development|PrintString "PLAYER ATTACK")
    (CallFunction|EnablePlayerUI)
    (else
      (for _array_element (Variables|Default|Getenemies)
        ;[1 0 0] DEBUG
        (Development|PrintString "ENEMY ATTACK")
        (CallFunction|EnemyAction)
        (CallFunction|UpdatePartyMembers))
      (CallFunction|PrepareNextRound))))

(event Custom|Start%20Fight
  (if (== (Variables|Default|GetisPartiesTurn) true)
    ;[1 0 0] DEBUG
    (Development|PrintString "PLAYER ATTACK")
    (CallFunction|EnablePlayerUI)
    (else
      (for _array_element (Variables|Default|Getenemies)
        ;[1 0 0] DEBUG
        (Development|PrintString "ENEMY ATTACK")
        (CallFunction|EnemyAction)
        (CallFunction|UpdatePartyMembers))
      (CallFunction|PrepareNextRound))))

(event Custom|End%20Fight
  (Widget|RemovefromParent (Variables|Default|GetfightUI))
  (Widget|RemovefromParent (Variables|Default|GetenemyUI))
  (for _array_element (Variables|/Game/Core/Characters/BP_PartyMembers.BP_PartyMembers_C|GetpartyMembers (Variables|Default|GetpartyMembers))
    (Utilities|IsValid _array_element
      (:Is%20Valid
        (Rendering|SetActorHiddenInGame _array_element true))))
  (CallFunction|SetIsFightStarted false)
  (Variables|/Script/Engine.PlayerController|SetbShowMouseCursor (Game|GetPlayerController 0) false)
  (bind _asbp_game_instance (Utilities|Casting|CastToBP_GameInstance (Game|GetGameInstance)))
  (Default|UpdateTicksAfterFight _asbp_game_instance)
  (bind _cart (Default|GetCart _asbp_game_instance))
  (Default|StartCartmodeAfterFight _cart)
  ;[1 0 0] Debug
  (Development|PrintString "Kampf vorbei")
  (Actor|DestroyActor))

(event Custom|Execute%20Char%20Fight%20Actions
  (for _index (range 0 (- (Utilities|Map|Length (Variables|Default|GetfightActions)) 1))
    (bind _output_get (Variables|Default|SetcurrentCharacter (Utilities|Array|Get(acopy) (Variables|/Game/Core/Characters/BP_PartyMembers.BP_PartyMembers_C|GetpartyMembers (Variables|Default|GetpartyMembers)) _index)))
    (Development|PrintString (Utilities|GetDisplayName _output_get))
    (Utilities|IsValid (.chosenenemy (.Value (Utilities|Map|Find (Variables|Default|GetfightActions) (Variables|Default|GetcurrentCharacter))))
      (:Is%20Valid
        (switch Utilities|FlowControl|Switch|SwitchonE_FightAction (.fightaction (.Value (Utilities|Map|Find (Variables|Default|GetfightActions) (Variables|Default|GetcurrentCharacter))))
          (:NewEnumerator0
            (Default|BaseAttack (Variables|Default|GetcurrentCharacter) (.chosenenemy (.Value (Utilities|Map|Find (Variables|Default|GetfightActions) (Variables|Default|GetcurrentCharacter))))))
          (:NewEnumerator1
            (Default|SpecialAttack (Variables|Default|GetcurrentCharacter) (.chosenenemy (.Value (Utilities|Map|Find (Variables|Default|GetfightActions) (Variables|Default|GetcurrentCharacter)))))
            (bind _currentweapon (Default|GetCurrentWeapon (Variables|Default|GetcurrentCharacter)))
            (bind _roundcounter (CallFunction|GetRoundCounter))
            (Default|SetLastUseSpecialAttack _currentweapon _roundcounter)
            (Default|SetSpecialAttackButtonInvalid (Variables|Default|GetfightUI) _index))
          (:NewEnumerator2
            (Default|Heal (Variables|Default|GetcurrentCharacter))))
        (Math|Integer|IncrementInt (Variables|Default|GetturnCounter)
          (:%20%20
            (Utilities|IsValid (.chosenenemy (.Value (Utilities|Map|Find (Variables|Default|GetfightActions) (Variables|Default|GetcurrentCharacter))))
              (:Is%20Valid
                (bind _health (Default|GetCurrentHealth (.chosenenemy (.Value (Utilities|Map|Find (Variables|Default|GetfightActions) (Variables|Default|GetcurrentCharacter))))))
                (bind _maxhealth (Default|GetMaxHealth (.chosenenemy (.Value (Utilities|Map|Find (Variables|Default|GetfightActions) (Variables|Default|GetcurrentCharacter))))))
                (Progress|SetPercent (Utilities|Array|Get(acopy) (Variables|/Game/UI/WBP_Enemies.WBP_Enemies_C|GetprogressBars (Variables|Default|GetenemyUI)) (Utilities|Array|FindItem (Variables|Default|Getenemies) (.chosenenemy (.Value (Utilities|Map|Find (Variables|Default|GetfightActions) (Variables|Default|GetcurrentCharacter)))))) (/ _health _maxhealth))
                (CallFunction|UpdateEnemies (.chosenenemy (.Value (Utilities|Map|Find (Variables|Default|GetfightActions) (Variables|Default|GetcurrentCharacter))))))))))))
  (Widget|SetIsEnabled (Variables|Default|GetfightUI) false)
  (CallFunction|PrepareNextRound))

(event Custom|Set%20Chosen%20Enemy
  (params (chosenEnemy :type Integer))
  (bind _output_get (Variables|Default|SetattackedEntity (Utilities|Array|Get(acopy) (Variables|Default|Getenemies) chosenEnemy)))
  (Utilities|Map|Add (Variables|Default|GetfightActions) (Variables|Default|GetcurrentCharacter) (Utilities|Struct|MakeS_FightAction (.fightaction (.Value (Utilities|Map|Find (Variables|Default|GetfightActions) (Variables|Default|GetcurrentCharacter)))) _output_get)))

(event Custom|Set%20Char%20Fight%20Action
  (params (chosenPlayer :type Integer) (fightAction :type E_FightAction%20Enum :default "NewEnumerator0"))
  (Variables|Default|SetcurrentCharacter (Utilities|Array|Get(acopy) (Variables|/Game/Core/Characters/BP_PartyMembers.BP_PartyMembers_C|GetpartyMembers (Variables|Default|GetpartyMembers)) chosenPlayer))
  (Utilities|Map|Add (Variables|Default|GetfightActions) (Variables|Default|GetcurrentCharacter) (Utilities|Struct|MakeS_FightAction fightAction (Utilities|Array|Get(acopy) (Variables|Default|Getenemies))))
  (bind _partymembers (Default|GetPartyMembers (Variables|Default|GetpartyMembers)))
  (if (== (Utilities|Map|Length (Variables|Default|GetfightActions)) (Utilities|Array|Length _partymembers))
    (Widget|SetIsEnabled (Variables|/Game/UI/WBP_Fight_PlayerAction.WBP_Fight_PlayerAction_C|GetB_ConfirmActions (Variables|Default|GetfightUI)) true)))

(event Custom|Trigger%20Fight
  ;[0.4 0.95 0.3] Prepare Fight
  (Variables|/Script/Engine.PlayerController|SetbShowMouseCursor (Game|GetPlayerController 0) true)
  (UserInterface|Viewport|AddtoViewport (Variables|Default|GetfightUI) 0)
  (UserInterface|Viewport|AddtoViewport (Variables|Default|GetenemyUI) 0)
  (CallFunction|SetPartyMembers)
  (CallFunction|UpdatePartyMembers)
  (CallFunction|SpawnPartyMembers)
  (CallFunction|SetRoundCounter)
  (Game|Player|SetViewTargetwithBlend (Game|GetPlayerController 0) (Components|GetOwner (Variables|Default|GetCamera)) 0.0 "VTBlend_Linear" 0.0 false)
  (CallFunction|CalculateRoundLength)
  (bind _ispartystarting (CallFunction|DecideStartingParty))
  (if _ispartystarting
    (CallFunction|SetIsPartiesTurn true)
    (else
      (CallFunction|SetIsPartiesTurn false)))
  (CallFunction|StartFight))

(event EventBeginPlay
  (Utilities|FlowControl|Sequence
    (:then_0
      (bind _returnvalue (UserInterface|CreateWidget "/Game/UI/WBP_Fight_PlayerAction.WBP_Fight_PlayerAction_C" (Game|GetPlayerController 0)))
      (Variables|Default|SetfightUI _returnvalue))
    (:then_1
      (EventDispatchers|BindEventtoCharSetFightAction (Variables|Default|GetfightUI) (delegate Custom|Set%20Char%20Fight%20Action)))
    (:then_2
      (EventDispatchers|BindEventtoCharConfirmFightActions (Variables|Default|GetfightUI) (delegate Custom|Execute%20Char%20Fight%20Actions)))
    (:then_3
      (CallFunction|AddPositions))
    (:then_4
      (CallFunction|AddEnemiesforFight))
    (:then_5
      (bind _returnvalue_2 (UserInterface|CreateWidget "/Game/UI/WBP_Enemies.WBP_Enemies_C" (Game|GetPlayerController 0)))
      (bind _output_get (Variables|Default|SetenemyUI _returnvalue_2))
      (bind _enemiesalive (CallFunction|GetEnemiesAlive))
      (Default|SetEnemyAmount _output_get _enemiesalive))
    (:then_6
      (EventDispatchers|BindEventtoSetChosenEnemy (Variables|Default|GetenemyUI) (delegate Custom|Set%20Chosen%20Enemy)))))

(fn ConstructionScript)

(fn GetIsPartiesTurn
  (return (Variables|Default|GetisPartiesTurn)))

(fn SetIsPartiesTurn
  (params (isPartyTurn :type Boolean))
  (Variables|Default|SetisPartiesTurn isPartyTurn)
  (return))

(fn GetRoundCounter
  (return (Variables|Default|GetroundCounter)))

(fn SetRoundCounter
  (params (roundCounter :type Integer))
  (Variables|Default|SetroundCounter roundCounter)
  (return))

(fn AddEnemy
  (params (newEnemy :type BP%20Base%20Enemy%20Object%20Reference))
  (Utilities|Array|Add (Variables|Default|Getenemies) newEnemy)
  (return))

(fn CalculateRoundLength
  (bind _enemiesalive (CallFunction|GetEnemiesAlive))
  (Variables|Default|SetroundLength (+ _enemiesalive (Utilities|Array|Length (Variables|/Game/Core/Characters/BP_PartyMembers.BP_PartyMembers_C|GetpartyMembers (Variables|Default|GetpartyMembers)))))
  (return))

(fn SetNextRound
  (bind _result (Math|Integer|IncrementInt (Variables|Default|GetroundCounter))
    (:%20%20
      (Variables|Default|SetroundCounter _result)
      (return))))

(fn DecideStartingParty
  (if (== (Math|Integer|%(Integer) (Math|Random|RandomInteger 1000) 2) 0)
    (return true)
    (else
      (return false))))

(fn EnemyAction
  (bind _currentenemy (CallFunction|GetCurrentEnemyObject))
  (Development|PrintString (Utilities|GetDisplayName _currentenemy))
  (Utilities|IsValid _currentenemy
    (:Is%20Valid
      (bind _currentweapon (Default|GetCurrentWeapon _currentenemy))
      (bind _output_get (LocalVariables|SetcurrentWeapon _currentweapon))
      (Development|PrintString (Utilities|GetDisplayName _output_get))
      (bind _health (Default|GetCurrentHealth _currentenemy))
      (bind _maxhealth (Default|GetMaxHealth _currentenemy))
      ;[1 1 1] less than 40% Health true?
      (if (<= _health (* _maxhealth 0.4))
        ;[1 0 0] heilen oder angreifen --> gewisse Chance zu heilen
        (Development|PrintString "Vielleicht heilen?")
        (if (== (Math|Integer|%(Integer) (Math|Random|RandomInteger 100) 10) 0)
          (bind _currentenemy_2 (CallFunction|GetCurrentEnemyObject))
          (Default|Heal _currentenemy_2)
          (Development|PrintString "HEILUNG")
          (else
            (if (== (Math|Integer|%(Integer) (Math|Random|RandomInteger 1000) 2) 0) :!label _label
              (bind _usecounter (Default|GetUseCounterSpecialAttack (LocalVariables|GetcurrentWeapon)))
              (if (== _usecounter 0)
                (bind _currentenemy_3 (CallFunction|GetCurrentEnemyObject :!label _label_2))
                (bind _chosenpartymember (CallFunction|ChooseRandomPartyMember))
                (Default|SpecialAttack _currentenemy_3 _chosenpartymember)
                (Default|SetLastUseSpecialAttack (LocalVariables|GetcurrentWeapon) (Variables|Default|GetroundCounter))
                (else
                  (bind _lastuse (Default|GetLastUseSpecialAttack (LocalVariables|GetcurrentWeapon)))
                  (bind _attackinterval (Default|GetAttackIntervalSpecialAttack (LocalVariables|GetcurrentWeapon)))
                  (if (<= (+ _lastuse _attackinterval) (Variables|Default|GetroundCounter))
                    (goto _label_2)
                    (else
                      (bind _currentenemy_4 (CallFunction|GetCurrentEnemyObject :!label _label_3))
                      (bind _chosenpartymember_2 (CallFunction|ChooseRandomPartyMember))
                      (Default|BaseAttack _currentenemy_4 _chosenpartymember_2)))))
              (else
                (goto _label_3)))))
        (else
          (goto _label)))
      (bind _result (Math|Integer|IncrementInt (Variables|Default|GetcurrentEnemyIndex))
        (:%20%20
          (Variables|Default|SetcurrentEnemyIndex _result)
          (if (== (Math|Integer|%(Integer) (Variables|Default|GetcurrentEnemyIndex) (Variables|Default|GetenemiesAlive)) 0)
            (Variables|Default|SetcurrentEnemyIndex 0))
          (Math|Integer|IncrementInt (Variables|Default|GetturnCounter)
            (:%20%20
              (return))))))
    (:Is%20Not%20Valid
      (return))))

(fn GetCurrentEnemyObject
  (return (Utilities|Array|Get(acopy) (Variables|Default|Getenemies) (Variables|Default|GetcurrentEnemyIndex))))

(fn EnablePlayerUI
  (Widget|SetIsEnabled (Variables|Default|GetfightUI) true)
  (return))

(fn AddEnemiesforFight
  (Rendering|SetVisibility (Variables|Default|GetBP_BaseCharacter_Bandit) false false)
  (for _index (range 0 (- (Math|Random|RandomIntegerinRange 1 4) 1))
    (CallFunction|IncreaseEnemiesAlive)
    (bind _returnvalue (Game|SpawnActorfromClass "/Game/Core/Characters/BP_BaseEnemy_Bandit.BP_BaseEnemy_Bandit_C" (Utilities|Array|Get(acopy) (Variables|Default|GetenemyPositions) _index) "Undefined" "MultiplyWithRoot" 0 0))
    (CallFunction|AddEnemy _returnvalue)
    (bind _returnvalue_2 (Game|SpawnActorfromClass "/Game/Core/Fight/BP_BaseWeapon.BP_BaseWeapon_C" (Math|Transform|MakeTransform "0, 0, 0") "Undefined" "MultiplyWithRoot" 0 0))
    (Default|SetCurrentWeapon _returnvalue _returnvalue_2))
  (return))

(fn SetPartyMembers
  (bind _asbp_game_instance (Utilities|Casting|CastToBP_GameInstance (Game|GetGameInstance)))
  (bind _partymembers (Default|GetPartyMembers _asbp_game_instance))
  (Variables|Default|SetpartyMembers _partymembers)
  (return))

(fn GetIsFightStarted
  (return (Variables|Default|GetisFightStarted)))

(fn SetIsFightStarted
  (params (isFightStarted :type Boolean))
  (Variables|Default|SetisFightStarted isFightStarted)
  (return))

(fn SwitchTurn
  (bind _ispartiesturn (CallFunction|GetIsPartiesTurn))
  (CallFunction|SetIsPartiesTurn (not _ispartiesturn))
  (return))

(fn PrepareNextRound
  (Utilities|Map|Clear (Variables|Default|GetfightActions))
  (Widget|SetIsEnabled (Variables|/Game/UI/WBP_Fight_PlayerAction.WBP_Fight_PlayerAction_C|GetB_ConfirmActions (Variables|Default|GetfightUI)) false)
  (bind _isonepartydown (CallFunction|CheckDeath))
  (if _isonepartydown
    (CallFunction|EndFight)
    (else
      (CallFunction|SwitchTurn)
      (CallFunction|CalculateRoundLength)
      (CallFunction|UpdatePlayerSpecialAttackButtons)
      (CallFunction|SetNextRound)
      (CallFunction|BeginNextRound)))
  (return))

(fn UpdateEnemies
  (params (deadEnemy :type BP%20Base%20Enemy%20Object%20Reference))
  (bind _enemies (Variables|Default|Getenemies))
  (bind _isdead (Default|CheckDeath deadEnemy))
  (if _isdead
    (CallFunction|DespawnDeadEnemy (Utilities|Array|Get(acopy) _enemies (Utilities|Array|FindItem _enemies deadEnemy)))
    (CallFunction|DecreaseEnemiesAlive)
    (return)))

(fn DespawnDeadEnemy
  (params (deadEnemy :type BP%20Base%20Enemy%20Object%20Reference))
  (Widget|SetVisibility (Utilities|Array|Get(acopy) (Variables|/Game/UI/WBP_Enemies.WBP_Enemies_C|GetprogressBars (Variables|Default|GetenemyUI)) (Utilities|Array|FindItem (Variables|Default|Getenemies) deadEnemy)) "Hidden")
  (bind _currentweapon (Default|GetCurrentWeapon deadEnemy))
  (Actor|DestroyActor _currentweapon)
  (Actor|DestroyActor deadEnemy)
  (return))

(fn CheckDeath
  (LocalVariables|SetalivePartyMember 0)
  (LocalVariables|SetaliveEnemies 0)
  (for (_ _array_index) (Variables|/Game/Core/Characters/BP_PartyMembers.BP_PartyMembers_C|GetpartyMembers (Variables|Default|GetpartyMembers))
    (bind _isdead (Default|CheckDeath (Utilities|Array|Get(acopy) (Variables|/Game/Core/Characters/BP_PartyMembers.BP_PartyMembers_C|GetpartyMembers (Variables|Default|GetpartyMembers)) _array_index)))
    (if (not _isdead)
      (bind _result (Math|Integer|IncrementInt (LocalVariables|GetalivePartyMember))
        (:%20%20
          (LocalVariables|SetalivePartyMember _result)))))
  (for _array_element (Variables|Default|Getenemies)
    (Utilities|IsValid _array_element
      (:Is%20Valid
        (bind _isdead_2 (Default|CheckDeath _array_element))
        (if (not _isdead_2)
          (bind _result_2 (Math|Integer|IncrementInt (LocalVariables|GetaliveEnemies))
            (:%20%20
              (LocalVariables|SetaliveEnemies _result_2)))))))
  (if (== (LocalVariables|GetalivePartyMember) 0)
    _
    (elif (== (LocalVariables|GetaliveEnemies) 0)
      _
      (else
        (return false))))
  (Development|PrintString "EINER TOT")
  (return true))

(fn AddPositions
  (bind _enemypositions (Variables|Default|GetenemyPositions))
  (bind _characterpositions (Variables|Default|GetcharacterPositions))
  (Utilities|Array|Add _enemypositions (Transformation|GetWorldTransform (Variables|Default|GetPosition1)))
  (Utilities|Array|Add _enemypositions (Transformation|GetWorldTransform (Variables|Default|GetPosition2)))
  (Utilities|Array|Add _enemypositions (Transformation|GetWorldTransform (Variables|Default|GetPosition3)))
  (Utilities|Array|Add _enemypositions (Transformation|GetWorldTransform (Variables|Default|GetPosition4)))
  (Utilities|Array|Add _characterpositions (Transformation|GetWorldTransform (Variables|Default|GetPosition5)))
  (Utilities|Array|Add _characterpositions (Transformation|GetWorldTransform (Variables|Default|GetPosition6)))
  (Utilities|Array|Add _characterpositions (Transformation|GetWorldTransform (Variables|Default|GetPosition7)))
  (Utilities|Array|Add _characterpositions (Transformation|GetWorldTransform (Variables|Default|GetPosition8)))
  (return))

(fn SpawnPartyMembers
  (for (_array_element _array_index) (Variables|/Game/Core/Characters/BP_PartyMembers.BP_PartyMembers_C|GetpartyMembers (Variables|Default|GetpartyMembers))
    (Transformation|SetActorTransform _array_element (Utilities|Array|Get(acopy) (Variables|Default|GetcharacterPositions) _array_index))
    (Rendering|SetActorHiddenInGame _array_element false))
  (return))

(fn UpdatePartyMembers
  (for (_array_element _array_index) (Variables|/Game/Core/Characters/BP_PartyMembers.BP_PartyMembers_C|GetpartyMembers (Variables|Default|GetpartyMembers))
    (bind _health (Default|GetCurrentHealth _array_element))
    (if (> _health 0.0)
      (bind _maxhealth (Default|GetMaxHealth _array_element))
      (Progress|SetPercent (Utilities|Array|Get(acopy) (Variables|/Game/UI/WBP_Fight_PlayerAction.WBP_Fight_PlayerAction_C|GetprogressBars (Variables|Default|GetfightUI)) _array_index) (/ _health _maxhealth))
      (else
        (Variables|/Game/Core/Characters/BP_BaseEntity.BP_BaseEntity_C|SetisDead _array_element true)
        (Development|PrintString "TOT")
        (Widget|SetVisibility (Utilities|Array|Get(acopy) (Variables|/Game/UI/WBP_Fight_PlayerAction.WBP_Fight_PlayerAction_C|GetprogressBars (Variables|Default|GetfightUI)) _array_index) "Hidden")
        (bind _asbp_game_instance (Utilities|Casting|CastToBP_GameInstance (Game|GetGameInstance)))
        (bind _partymembers (Default|GetPartyMembers _asbp_game_instance))
        (Utilities|Array|RemoveItem (Variables|/Game/Core/Characters/BP_PartyMembers.BP_PartyMembers_C|GetpartyMembers _partymembers) _array_element))))
  (return))

(fn SetEnemiesAlive
  (params (enemiesAlive :type Integer))
  (CallFunction|SetEnemiesAlive enemiesAlive)
  (return))

(fn GetEnemiesAlive
  (return (Variables|Default|GetenemiesAlive)))

(fn DecreaseEnemiesAlive
  (bind _result (Math|Integer|DecrementInt (Variables|Default|GetenemiesAlive))
    (:%20%20
      (Variables|Default|SetenemiesAlive _result)
      (return))))

(fn GetPartyMembers
  (return (Variables|Default|GetpartyMembers)))

(fn UpdatePlayerSpecialAttackButtons
  (if (> (Variables|Default|GetroundCounter) 0)
    (bind _partymembers (Default|GetPartyMembers (Variables|Default|GetpartyMembers)))
    (for (_array_element _array_index) _partymembers
      (bind _currentweapon (Default|GetCurrentWeapon _array_element))
      (bind _isusesleft (Default|CheckUsesLeftSpecialAttack _currentweapon))
      (if _isusesleft
        (bind _lastuse (Default|GetLastUseSpecialAttack _currentweapon))
        (bind _attackinterval (Default|GetAttackIntervalSpecialAttack _currentweapon))
        (Development|PrintString (Utilities|String|ToString(Integer) (+ _lastuse _attackinterval)))
        (if (<= (+ _lastuse _attackinterval) (Variables|Default|GetroundCounter))
          (Default|SetSpecialAttackButtonValid (Variables|Default|GetfightUI) _array_index))))
    (return)))

(fn IncreaseEnemiesAlive
  (bind _result (Math|Integer|IncrementInt (Variables|Default|GetenemiesAlive))
    (:%20%20
      (Variables|Default|SetenemiesAlive _result)
      (return))))

(fn ChooseRandomPartyMember
  (return (Utilities|Array|Get(acopy) (Variables|/Game/Core/Characters/BP_PartyMembers.BP_PartyMembers_C|GetpartyMembers (Variables|Default|GetpartyMembers)) (Math|Integer|%(Integer) (Math|Random|RandomInteger 1000) (Utilities|Array|Length (Variables|/Game/Core/Characters/BP_PartyMembers.BP_PartyMembers_C|GetpartyMembers (Variables|Default|GetpartyMembers)))))))