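; Base character Blueprint that handles food, starvation, weapon swapping and weapon attack animations, plus a heal counter.
; Tick clamps Food at zero and sets IsStarving, while IncrementFood caps it at MaxFood.
; Weapon changes map the item's type to a weapon class, destroy the current weapon, then spawn a replacement with the item's stats on WeaponSocket.
; TriggerWeaponAnimation switches on the current weapon type to call the matching BP_Anim_HumanChar trigger.
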(event EventBeginPlay)

(event Collision|EventActorBeginOverlap
  (params (OtherActor :type Actor%20Object%20Reference)))

(event EventTick
  (params (DeltaSeconds :type Float%20%28single-precision%29))
  (if (<= (Variables|Default|Getfood) 0.0)
    (Variables|Default|Setfood 0.0)
    (Variables|Default|SetisStarving true)
    (else
      (Variables|Default|SetisStarving false))))

(fn ConstructionScript)

(fn GetFood
  (return (Variables|Default|Getfood)))

(fn SetFood
  (params (newFood :type Float%20%28double-precision%29))
  (Variables|Default|Setfood newFood)
  (return))

(fn GetAnimationBlueprint
  (bind _asbp_anim_human_char (Utilities|Casting|CastToBP_Anim_HumanChar (Components|SkeletalMesh|GetAnimInstance (Variables|Default|GetSkeletalMesh))))
  (return _asbp_anim_human_char))

(fn TriggerWeaponAnimation
  (params (animBlueprint :type BP%20Anim%20Human%20Char%20Object%20Reference))
  (switch Utilities|FlowControl|Switch|SwitchonE_Weapon (Variables|/Game/Core/Events/Fight/Weapons/BP_BaseWeapon.BP_BaseWeapon_C|GetweaponType (Variables|Default|GetcurrentWeapon))
    (:NewEnumerator0
      (Default|TriggerAnimAxe animBlueprint))
    (:NewEnumerator1
      (Default|TriggerAnimBow animBlueprint))
    (:NewEnumerator2
      (Default|TriggerAnimCrossbow animBlueprint))
    (:NewEnumerator3
      (Default|TriggerAnimDagger animBlueprint))
    (:NewEnumerator4
      (Default|TriggerAnimBook animBlueprint))
    (:NewEnumerator5
      (Default|TriggerAnimWand animBlueprint))
    (:NewEnumerator6
      (Default|TriggerAnimShield animBlueprint))
    (:NewEnumerator7
      (Default|TriggerAnimStick animBlueprint))
    (:NewEnumerator8
      (Default|TriggerAnimSword animBlueprint)))
  (return))

(fn IncrementFood
  (params (food :type Float%20%28double-precision%29))
  (bind _maxfood (Variables|Default|GetmaxFood))
  (bind _output_get (Variables|Default|Setfood (+ food (Variables|Default|Getfood))))
  (if (> _output_get _maxfood)
    (Variables|Default|Setfood _maxfood)
    (return)
    (else
      (return))))

(fn ChangeWeaponwithWeaponType
  (params (weaponItem :type BP%20Item%20Weapon%20Object%20Reference))
  (switch Utilities|FlowControl|Switch|SwitchonE_Weapon (Default|GetWeaponType weaponItem)
    (:NewEnumerator0
      (Variables|Default|SetweaponClass "/Game/Core/Events/Fight/Weapons/BP_BaseWeapon_Axe.BP_BaseWeapon_Axe_C"))
    (:NewEnumerator1
      (Variables|Default|SetweaponClass "/Game/Core/Events/Fight/Weapons/BP_BaseWeapon_Bow.BP_BaseWeapon_Bow_C"))
    (:NewEnumerator2
      (Variables|Default|SetweaponClass "/Game/Core/Events/Fight/Weapons/BP_BaseWeapon_Crossbow.BP_BaseWeapon_Crossbow_C"))
    (:NewEnumerator3
      (Variables|Default|SetweaponClass "/Game/Core/Events/Fight/Weapons/BP_BaseWeapon_Dagger.BP_BaseWeapon_Dagger_C"))
    (:NewEnumerator4
      (Variables|Default|SetweaponClass "/Game/Core/Events/Fight/Weapons/BP_BaseWeapon_MagicBook.BP_BaseWeapon_MagicBook_C"))
    (:NewEnumerator5
      (Variables|Default|SetweaponClass "/Game/Core/Events/Fight/Weapons/BP_BaseWeapon_MagicWand.BP_BaseWeapon_MagicWand_C"))
    (:NewEnumerator6
      (Variables|Default|SetweaponClass "/Game/Core/Events/Fight/Weapons/BP_BaseWeapon_Shield.BP_BaseWeapon_Shield_C"))
    (:NewEnumerator7
      (Variables|Default|SetweaponClass "/Game/Core/Events/Fight/Weapons/BP_BaseWeapon_Stick.BP_BaseWeapon_Stick_C"))
    (:NewEnumerator8
      (Variables|Default|SetweaponClass "/Game/Core/Events/Fight/Weapons/BP_BaseWeapon_Sword.BP_BaseWeapon_Sword_C")))
  (bind _weapon (CallFunction|SpawnandAttachChangedWeapon (Variables|Default|GetweaponClass) weaponItem))
  (CallFunction|SetCurrentWeapon _weapon))

(fn SpawnandAttachChangedWeapon
  (params (weaponClass :type BP%20Base%20Weapon%20Class%20Reference) (weaponItem :type BP%20Item%20Weapon%20Object%20Reference))
  (bind _currentweapon (CallFunction|GetCurrentWeapon))
  (Actor|DestroyActor _currentweapon)
  (bind _returnvalue (Game|SpawnActorfromClass weaponClass (Math|Transform|MakeTransform "0, 0, 0" "180.000000,0.000000,0.000000" "0.010000,0.010000,0.010000") "Undefined" "MultiplyWithRoot" 0 0))
  (Variables|/Game/Core/Events/Fight/Weapons/BP_BaseWeapon.BP_BaseWeapon_C|SetmaxUsesSpecialAttack _returnvalue (Default|GetMaxUsesSpecialAttack weaponItem))
  (Variables|/Game/Core/Events/Fight/Weapons/BP_BaseWeapon.BP_BaseWeapon_C|SetattackIntervalSpecialAttack _returnvalue (Default|GetAttackIntervalSpecialAttack weaponItem))
  (Variables|/Game/Core/Events/Fight/Weapons/BP_BaseWeapon.BP_BaseWeapon_C|SetweaponType _returnvalue (Default|GetWeaponType weaponItem))
  (Variables|/Game/Core/Events/Fight/Weapons/BP_BaseWeapon.BP_BaseWeapon_C|SetdamageBaseAttack _returnvalue (Default|GetDamageBaseAttack weaponItem))
  (Variables|/Game/Core/Events/Fight/Weapons/BP_BaseWeapon.BP_BaseWeapon_C|SetdamageSpecialAttack _returnvalue (Default|GetDamageSpecialAttack weaponItem))
  (Variables|/Game/Core/Events/Fight/Weapons/BP_BaseWeapon.BP_BaseWeapon_C|SetweaponName _returnvalue (Default|GetItemName weaponItem))
  (Transformation|AttachComponentToComponent _returnvalue (Variables|Default|GetSkeletalMesh) "WeaponSocket" "KeepRelative" "KeepRelative" "KeepRelative" true)
  (return _returnvalue))

(fn IncreaseHealCounter
  (bind _result (Math|Integer|IncrementInt (Variables|Default|GethealCounter))
    (:%20%20
      (Variables|Default|SethealCounter _result))))