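; BP_Startmenu runs the start menu, playing music through BP_GameInstance when play begins.
; If the game has not started, it shows the cursor and WBP_Startmenu, then sets the view target to its camera's owner.
; The widget's start event opens Ouroboros_Gameplay with a game mode override in the options, clears the menu-open flag and hides the cursor.
; Its leave event quits the game.
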(event Custom|StartGame
  (Game|OpenLevel(byName) "Ouroboros_Gameplay" true "?Game=/Game/Core/General/BP_MyGameMode.BP_MyGameMode_C")
  (bind _asbp_game_instance (Utilities|Casting|CastToBP_GameInstance (Game|GetGameInstance)))
  (Variables|/Game/Core/General/BP_GameInstance.BP_GameInstance_C|SetisStartMenuOpen _asbp_game_instance false)
  (Variables|/Script/Engine.PlayerController|SetbShowMouseCursor (Game|GetPlayerController 0) false))

(event Custom|Leave%20Game
  (Game|QuitGame 0 "Quit" false))

(event EventBeginPlay
  (bind _returnvalue (Game|GetPlayerController 0))
  (bind _asbp_game_instance (Utilities|Casting|CastToBP_GameInstance (Game|GetGameInstance)))
  (Default|PlayMusic _asbp_game_instance)
  (if (not (Variables|/Game/Core/General/BP_GameInstance.BP_GameInstance_C|GetisGameStarted _asbp_game_instance))
    (Variables|/Script/Engine.PlayerController|SetbShowMouseCursor _returnvalue true)
    (bind _returnvalue_2 (UserInterface|CreateWidget "/Game/UI/WBP_Startmenu.WBP_Startmenu_C" _returnvalue))
    (bind _output_get (Variables|Default|SetstartMenuUI _returnvalue_2))
    (UserInterface|Viewport|AddtoViewport _output_get 0)
    (EventDispatchers|BindEventtoStartGame (Variables|Default|GetstartMenuUI) (delegate Custom|StartGame))
    (EventDispatchers|BindEventtoLeaveGame (Variables|Default|GetstartMenuUI) (delegate Custom|Leave%20Game))
    (Game|Player|SetViewTargetwithBlend (Game|GetPlayerController 0) (Components|GetOwner (Variables|Default|GetCamera)) 0.0 "VTBlend_Linear" 0.0 false)))

(fn ConstructionScript)