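; BP_TickManager is an actor that counts game ticks based on spline distance while the cart is driving.
; It finds BP_SplineMovement on BeginPlay, then each frame checks whether its truncated SplineLength modulo 250 falls within 0 to 3, a window that tolerates rounding errors.
; A match increments TickCounter after a short Delay for more natural pacing and prints the count for debugging.
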(event EventBeginPlay
  ;[1 1 1] get SplineMovement reference
  (Utilities|FlowControl|Sequence
    (:then_1
      (bind _returnvalue (Actor|GetActorOfClass "/Game/Ouroboros/Core/BP_SplineMovement.BP_SplineMovement_C"))
      (Variables|Default|SetsplineMovement _returnvalue))))

(event EventTick
  (params (DeltaSeconds :type Float%20%28single-precision%29))
  (bind _splinemovement (Variables|Default|GetsplineMovement))
  (bind _splinelength (Variables|/Game/Ouroboros/Core/BP_SplineMovement.BP_SplineMovement_C|GetsplineLength _splinemovement))
  (bind _returnvalue (Math|Float|Truncate _splinelength))
  (bind _returnvalue_2 (Math|Integer|%(Integer) _returnvalue 250))
  (if (and (Variables|/Game/Ouroboros/Core/BP_Cart.BP_Cart_C|GetisDriving (Variables|/Game/Ouroboros/Core/BP_SplineMovement.BP_SplineMovement_C|Getcart (Variables|Default|GetsplineMovement))) (and (<= _returnvalue_2 3) (>= _returnvalue_2 0)))
    ;[1 1 1 1 12] needs to be slightly delayed --> tick increments feel more natural
    (Utilities|FlowControl|Delay 0.1)
    ;[1 1 1] increment tickCounter
    (bind _output_get (Variables|Default|SettickCounter (+ (Variables|Default|GettickCounter) 1)))
    ;[1 0 0] DEBUG
    (Development|PrintString (Utilities|String|ToString(Integer) _output_get))))

(fn ConstructionScript)