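; BP_BaseEntity is a base character Blueprint holding combat state: health, defense, current weapon, and death and action flags, exposed through getters and setters.
; BaseAttack and SpecialAttack delegate to the current weapon, raising a matching flag only for the duration of the call.
; Heal adds a fixed amount capped at max health, and CheckDeath marks the entity dead at zero health or below.
; The event graph is empty, so all logic runs through called functions.
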(event EventBeginPlay)

(event Collision|EventActorBeginOverlap
  (params (OtherActor :type Actor%20Object%20Reference)))

(event EventTick
  (params (DeltaSeconds :type Float%20%28single-precision%29)))

(fn ConstructionScript)

(fn GetCurrentHealth
  (return (Variables|Default|GetcurrentHealth)))

(fn GetDefense
  (return (Variables|Default|Getdefense)))

(fn SetCurrentHealth
  (params (newHealth :type Float%20%28double-precision%29))
  (Variables|Default|SetcurrentHealth newHealth)
  (return))

(fn GetCurrentWeapon
  (return (Variables|Default|GetcurrentWeapon)))

(fn SetCurrentWeapon
  (params (newWeapon :type BP%20Base%20Weapon%20Object%20Reference))
  (bind _output_get (Variables|Default|SetcurrentWeapon newWeapon))
  (Variables|/Game/Core/Fight/Weapons/BP_BaseWeapon.BP_BaseWeapon_C|SetweaponType _output_get (Variables|/Game/Core/Fight/Weapons/BP_BaseWeapon.BP_BaseWeapon_C|GetweaponType newWeapon))
  (return))

(fn GetMaxHealth
  (return (Variables|Default|GetmaxHealth)))

(fn Heal
  (Variables|Default|SetisHealing true)
  (bind _health (CallFunction|GetCurrentHealth))
  (bind _maxhealth (CallFunction|GetMaxHealth))
  (if (> (+ _health 2e+01) _maxhealth)
    (CallFunction|SetCurrentHealth _maxhealth)
    (else
      (CallFunction|SetCurrentHealth (+ _health 2e+01))))
  (Variables|Default|SetisHealing false)
  (return))

(fn SetDefense
  (params (newDefense :type Float%20%28double-precision%29))
  (Variables|Default|Setdefense newDefense)
  (return))

(fn BaseAttack
  (params (attackedEntity :type BP%20Base%20Entity%20Object%20Reference))
  (Variables|Default|SetisUsingBaseAttack true)
  (Default|BaseAttack (Variables|Default|GetcurrentWeapon) attackedEntity)
  (Variables|Default|SetisUsingBaseAttack false)
  (return))

(fn SpecialAttack
  (params (attackedEntity :type BP%20Base%20Entity%20Object%20Reference))
  (Variables|Default|SetisUsingSpecialAttack true)
  (Default|SpecialAttack (Variables|Default|GetcurrentWeapon) attackedEntity)
  (Variables|Default|SetisUsingSpecialAttack false)
  (return))

(fn CheckDeath
  (bind _health (CallFunction|GetCurrentHealth))
  (if (<= _health 0.0)
    (Variables|Default|SetisDead true)
    (Development|PrintString "CHAR TOT")
    (return true)
    (else
      (return false))))

(fn GetIsUsingSpecialAttack
  (return (Variables|Default|GetisUsingSpecialAttack)))

(fn GetIsUsingBaseAttack
  (return (Variables|Default|GetisUsingBaseAttack)))

(fn GetIsHealing
  (return (Variables|Default|GetisHealing)))

(fn SetIsUsingSpecialAttack
  (params (isUsingSpecialAttack :type Boolean))
  (Variables|Default|SetisUsingSpecialAttack isUsingSpecialAttack)
  (return))

(fn SetIsUsingBaseAttack
  (params (isUsingBaseAttack :type Boolean))
  (Variables|Default|SetisUsingBaseAttack isUsingBaseAttack)
  (return))

(fn SetIsHealing
  (params (isHealing :type Boolean))
  (Variables|Default|SetisHealing isHealing)
  (return))

(fn GetIsDeath
  (return (Variables|Default|GetisDead)))