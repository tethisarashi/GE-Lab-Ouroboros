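; BP_POICamera is a point-of-interest camera marker that moves the Cart's camera to its own POICamera viewpoint.
; MoveCameraToPOI gets the Cart through BP_GameInstance and saves the camera's relative transform in CartCamTransform before moving it.
; A timeline then lerps the camera's world transform toward POICamera, blending from its current transform on each update rather than from a fixed start.
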(event Custom|MoveCameraToPOI
  (bind _asbp_game_instance (Utilities|Casting|CastToBP_GameInstance (Game|GetGameInstance)))
  (Variables|/Game/Core/BP_Cart.BP_Cart_C|SetcartCamTransform (Variables|/Game/Core/General/BP_GameInstance.BP_GameInstance_C|Getcart _asbp_game_instance) (Transformation|GetRelativeTransform (Variables|/Game/Core/BP_Cart.BP_Cart_C|GetCamera (Variables|/Game/Core/General/BP_GameInstance.BP_GameInstance_C|Getcart _asbp_game_instance))))
  (bind _newtrack_0 (Timeline|Timeline Play)
    (:Update
      (Transformation|SetWorldTransform (Variables|/Game/Core/BP_Cart.BP_Cart_C|GetCamera (Variables|/Game/Core/General/BP_GameInstance.BP_GameInstance_C|Getcart _asbp_game_instance)) (Math|Transform|Lerp(Transform) (Transformation|GetWorldTransform (Variables|/Game/Core/BP_Cart.BP_Cart_C|GetCamera (Variables|/Game/Core/General/BP_GameInstance.BP_GameInstance_C|Getcart _asbp_game_instance))) (Transformation|GetWorldTransform (Variables|Default|GetPOICamera)) _newtrack_0) false false))))

(fn ConstructionScript)