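; Beggar encounter event, shown as a peasant NPC, that asks the player for a random item and gives another random one in exchange.
; BeginPlay picks the desired item through the main inventory and binds the beggar widget's give and leave callbacks.
; StartEvent shows the widget and enables its buttons based on whether the player holds that item.
; Giving swaps the item and plays the quest sound, while only leaving calls FinishEvent to destroy the actor.
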(event Custom|GiveItem
  (CallFunction|GiveDesiredItem)
  (bind _asbp_game_instance (Utilities|Casting|CastToBP_GameInstance (Game|GetGameInstance)))
  (Default|PlayQuestSound (Default|GetSoundManager _asbp_game_instance)))

(event Custom|Leave
  (CallFunction|FinishEvent))

(event EventBeginPlay
  (Variables|Default|SetvisibleMesh "/Game/Entity/Human/NPC/SK_Entity_NPC_Peasant2.SK_Entity_NPC_Peasant2")
  (bind _returnvalue (UserInterface|CreateWidget "/Game/UI/Events/WBP_BeggarEvent.WBP_BeggarEvent_C" (Game|GetPlayerController 0)))
  (Variables|Default|Setui _returnvalue)
  (bind _asbp_game_instance (Utilities|Casting|CastToBP_GameInstance (Game|GetGameInstance)))
  (bind _item (Default|GetRandomItem (Variables|/Game/Core/General/BP_GameInstance.BP_GameInstance_C|GetmainInventory _asbp_game_instance)))
  (bind _output_get (Variables|Default|SetdesiredItem _item))
  (Variables|/Game/UI/Events/WBP_BeggarEvent.WBP_BeggarEvent_C|SetdesiredItemName (Variables|Default|Getui) (Default|GetItemName _output_get))
  (EventDispatchers|BindEventtoGiveItem (Variables|Default|Getui) (delegate Custom|GiveItem))
  (EventDispatchers|BindEventtoLeave (Variables|Default|Getui) (delegate Custom|Leave))
  (|CallParentFunction))

(fn ConstructionScript
  (|CallParentFunction))

(fn StartEvent
  (bind _ui (Variables|Default|Getui))
  (|CallParentFunction)
  (UserInterface|Viewport|AddtoViewport (Variables|Default|Getui) 0)
  (bind _asbp_game_instance (Utilities|Casting|CastToBP_GameInstance (Game|GetGameInstance)))
  (Default|PlayScrollSound (Default|GetSoundManager _asbp_game_instance))
  (Variables|/Script/Engine.PlayerController|SetbShowMouseCursor (Game|GetPlayerController 0) true)
  (bind _asbp_game_instance_2 (Utilities|Casting|CastToBP_GameInstance (Game|GetGameInstance)))
  (bind (_isitemfound _founditem) (Default|CheckIteminInventory (Variables|/Game/Core/General/BP_GameInstance.BP_GameInstance_C|GetmainInventory _asbp_game_instance_2) (Variables|Default|GetdesiredItem)))
  (Variables|Default|SetfoundItem _founditem)
  (if _isitemfound
    (Default|SetIDontHaveItButtonInvalid _ui)
    (Default|SetYesButtonValid _ui)
    (Default|SetNoButtonValid _ui)
    (else
      (Default|SetIDontHaveItButtonValid _ui)
      (Default|SetYesButtonInvalid _ui)
      (Default|SetNoButtonInvalid _ui))))

(fn FinishEvent
  (|CallParentFunction)
  (Widget|RemovefromParent (Variables|Default|Getui))
  (Variables|/Script/Engine.PlayerController|SetbShowMouseCursor (Game|GetPlayerController 0) false)
  (Actor|DestroyActor))

(fn GiveDesiredItem
  (bind _asbp_game_instance (Utilities|Casting|CastToBP_GameInstance (Game|GetGameInstance)))
  (Default|RemoveItem (Variables|/Game/Core/General/BP_GameInstance.BP_GameInstance_C|GetmainInventory _asbp_game_instance) (Variables|Default|GetfoundItem))
  (bind _item (Default|GetRandomItem (Variables|/Game/Core/General/BP_GameInstance.BP_GameInstance_C|GetmainInventory _asbp_game_instance)))
  (Default|TryAddItem (Variables|/Game/Core/General/BP_GameInstance.BP_GameInstance_C|GetmainInventory _asbp_game_instance) _item))