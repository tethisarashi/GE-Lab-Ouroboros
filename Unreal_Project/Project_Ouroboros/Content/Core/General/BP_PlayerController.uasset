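; Player controller that turns Enhanced Input actions into control of a spline-following cart: starting and stopping, three-lane steering, path choice and leaving POIs.
; It gets the cart and spline movement from the GameInstance, whose game state gates driving and POI exit.
; Four timelines lerp the cart's lateral offset between lanes, with cart flags blocking overlapping changes.
; Path choices swap the main spline, and leaving a POI blends back to the cart camera.
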(event Input|EnhancedActionEvents|EnhancedInputActionIA_DriveRight
  (params (ActionValue :type Float%20%28double-precision%29) (ElapsedSeconds :type Float%20%28double-precision%29) (TriggeredSeconds :type Float%20%28double-precision%29) (InputAction :type Input%20Action%20Object%20Reference :default "/Game/Core/Input/IA_DriveRight.IA_DriveRight"))
  (bind _cart (Variables|Default|Getcart))
  (bind _cart_2 (Variables|Default|Getcart))
  (bind _cart_3 (Variables|Default|Getcart))
  (bind _cart_4 (Variables|Default|Getcart))
  (bind _asbp_game_instance (Utilities|Casting|CastToBP_GameInstance (Game|GetGameInstance)))
  (if (Utilities|Enum|Equal(Enum) (Variables|/Game/Core/General/BP_GameInstance.BP_GameInstance_C|GetcurrentGameState _asbp_game_instance) "NewEnumerator0")
    ;[1 1 1] Trigger Animation
    (if (and (and (== (Variables|/Game/Core/BP_Cart.BP_Cart_C|GetisChoosingPath _cart_3) false) (== (Variables|/Game/Core/BP_Cart.BP_Cart_C|GetisDriving _cart_3) true)) (== (Variables|/Game/Core/BP_Cart.BP_Cart_C|GetisDrivingRight _cart_3) false))
      (Default|TriggerAnimRight _cart_4)
      ;[0.4 0.95 0.3] WASD Controls
      ;;[0.4 0.95 0.3] Input Event Driving Right
      (if (== (Variables|/Game/Core/BP_Cart.BP_Cart_C|GetisDriving _cart_4) true)
        (if (== (Variables|/Game/Core/BP_Cart.BP_Cart_C|GetisChangingLanes _cart_4) false)
          ;;;[1 1 1] Driving from left to middle --> driving right
          (if (and (== (Variables|/Game/Core/BP_Cart.BP_Cart_C|GetisDrivingLeft _cart_4) true) (== (Variables|/Game/Core/BP_Cart.BP_Cart_C|GetisDrivingRight _cart_4) false))
            (bind _newtrack_0 (Timeline|Timeline_FromLeftToRight PlayFromStart)
              (:Update
                (Variables|/Game/Core/BP_Cart.BP_Cart_C|Setoffset _cart (Math|Float|Lerp (* ActionValue (* (Variables|Default|GetpathWidthModifier) -1.0)) 0.0 _newtrack_0))
                (Variables|/Game/Core/BP_Cart.BP_Cart_C|SetisChangingLanes _cart true))
              (:Finished
                (Variables|/Game/Core/BP_Cart.BP_Cart_C|SetisDrivingLeft _cart false)
                (Variables|/Game/Core/BP_Cart.BP_Cart_C|SetisDrivingRight _cart false)
                (Variables|/Game/Core/BP_Cart.BP_Cart_C|SetisChangingLanes _cart false)))
            (else
              ;;;[1 1 1] Driving from middle to left --> driving left
              (if (and (== (Variables|/Game/Core/BP_Cart.BP_Cart_C|GetisDrivingLeft _cart_4) false) (== (Variables|/Game/Core/BP_Cart.BP_Cart_C|GetisDrivingRight _cart_4) false))
                (bind _newtrack_0_2 (Timeline|Timeline_FromMiddleToRight PlayFromStart)
                  (:Update
                    (Variables|/Game/Core/BP_Cart.BP_Cart_C|Setoffset _cart_2 (Math|Float|Lerp 0.0 (* ActionValue (Variables|Default|GetpathWidthModifier)) _newtrack_0_2))
                    (Variables|/Game/Core/BP_Cart.BP_Cart_C|SetisChangingLanes _cart_2 true))
                  (:Finished
                    (Variables|/Game/Core/BP_Cart.BP_Cart_C|SetisDrivingRight _cart_2 true)
                    (Variables|/Game/Core/BP_Cart.BP_Cart_C|SetisDrivingLeft _cart_2 false)
                    (Variables|/Game/Core/BP_Cart.BP_Cart_C|SetisChangingLanes _cart_2 false)))))))))))

(event Input|EnhancedActionEvents|EnhancedInputActionIA_ChooseLeftPath
  (params (ActionValue :type Boolean) (ElapsedSeconds :type Float%20%28double-precision%29) (TriggeredSeconds :type Float%20%28double-precision%29) (InputAction :type Input%20Action%20Object%20Reference :default "/Game/Core/Input/IA_ChooseLeftPath.IA_ChooseLeftPath"))
  (bind _splinemovement (Variables|Default|GetsplineMovement))
  (bind _cart (Variables|Default|Getcart))
  ;[0.4 0.95 0.3] Choose left/or right path
  (if (== (Variables|/Game/Core/BP_Cart.BP_Cart_C|GetisChoosingPath (Variables|Default|Getcart)) true)
    ;;[0.9645 0 1] ggf. Play Rate hier noch anpassen
    (Variables|/Game/Core/Movement/BP_SplineMovement.BP_SplineMovement_C|SetsplineMain _splinemovement (Variables|/Game/Core/Movement/BP_SplineMovement.BP_SplineMovement_C|GetsplineLeft _splinemovement))
    (Default|TriggerAnimLeft (Variables|Default|Getcart))
    (Default|DriveonChosenSpline (Variables|Default|GetsplineMovement))
    (Default|TriggerStartDriving _cart)
    (Utilities|FlowControl|Delay 0.2)
    (Variables|/Game/Core/BP_Cart.BP_Cart_C|SetisChoosingPath _cart false)))

(event Input|EnhancedActionEvents|EnhancedInputActionIA_StartDriving
  (params (ActionValue :type Boolean) (ElapsedSeconds :type Float%20%28double-precision%29) (TriggeredSeconds :type Float%20%28double-precision%29) (InputAction :type Input%20Action%20Object%20Reference :default "/Game/Core/Input/IA_StartDriving.IA_StartDriving"))
  ;[0.4 0.95 0.3] WASD Controls
  ;;[0.4 0.95 0.3] Input Events for start/stop driving --> triggered in cart
  (bind _asbp_game_instance (Utilities|Casting|CastToBP_GameInstance (Game|GetGameInstance)))
  (if (Utilities|Enum|Equal(Enum) (Variables|/Game/Core/General/BP_GameInstance.BP_GameInstance_C|GetcurrentGameState _asbp_game_instance) "NewEnumerator0")
    (Default|TriggerStartDriving (Variables|Default|Getcart))))

(event Input|EnhancedActionEvents|EnhancedInputActionIA_StopDriving
  (params (ActionValue :type Boolean) (ElapsedSeconds :type Float%20%28double-precision%29) (TriggeredSeconds :type Float%20%28double-precision%29) (InputAction :type Input%20Action%20Object%20Reference :default "/Game/Core/Input/IA_StopDriving.IA_StopDriving"))
  (bind _cart (Variables|Default|Getcart))
  ;[0.4 0.95 0.3] WASD Controls
  ;;[0.4 0.95 0.3] Input Events for start/stop driving --> triggered in cart
  (bind _asbp_game_instance (Utilities|Casting|CastToBP_GameInstance (Game|GetGameInstance)))
  (if (Utilities|Enum|Equal(Enum) (Variables|/Game/Core/General/BP_GameInstance.BP_GameInstance_C|GetcurrentGameState _asbp_game_instance) "NewEnumerator0")
    (if (not (Variables|/Game/Core/BP_Cart.BP_Cart_C|GetisChangingLanes _cart))
      (Default|TriggerStopDriving _cart))))

(event Input|EnhancedActionEvents|EnhancedInputActionIA_ChooseRightPath
  (params (ActionValue :type Boolean) (ElapsedSeconds :type Float%20%28double-precision%29) (TriggeredSeconds :type Float%20%28double-precision%29) (InputAction :type Input%20Action%20Object%20Reference :default "/Game/Core/Input/IA_ChooseRightPath.IA_ChooseRightPath"))
  (bind _splinemovement (Variables|Default|GetsplineMovement))
  (bind _cart (Variables|Default|Getcart))
  ;[0.4 0.95 0.3] Choose left/or right path
  (if (== (Variables|/Game/Core/BP_Cart.BP_Cart_C|GetisChoosingPath (Variables|Default|Getcart)) true)
    ;;[0.9645 0 1] ggf. Play Rate hier noch anpassen
    (Variables|/Game/Core/Movement/BP_SplineMovement.BP_SplineMovement_C|SetsplineMain _splinemovement (Variables|/Game/Core/Movement/BP_SplineMovement.BP_SplineMovement_C|GetsplineRight _splinemovement))
    (Default|TriggerAnimRight (Variables|Default|Getcart))
    (Default|DriveonChosenSpline (Variables|Default|GetsplineMovement))
    (Default|TriggerStartDriving _cart)
    (Utilities|FlowControl|Delay 0.2)
    (Variables|/Game/Core/BP_Cart.BP_Cart_C|SetisChoosingPath _cart false)))

(event Input|EnhancedActionEvents|EnhancedInputActionIA_LeavePOI
  (params (ActionValue :type Boolean) (ElapsedSeconds :type Float%20%28double-precision%29) (TriggeredSeconds :type Float%20%28double-precision%29) (InputAction :type Input%20Action%20Object%20Reference :default "/Game/Core/Input/IA_LeavePOI.IA_LeavePOI"))
  (bind _asbp_game_instance (Utilities|Casting|CastToBP_GameInstance (Game|GetGameInstance)))
  (if (Utilities|Enum|Equal(Enum) (Variables|/Game/Core/General/BP_GameInstance.BP_GameInstance_C|GetcurrentGameState _asbp_game_instance) "NewEnumerator1")
    (Game|Player|SetViewTargetwithBlend (Game|GetPlayerController 0) (Components|GetOwner (Variables|/Game/Core/BP_Cart.BP_Cart_C|GetCamera (Variables|Default|Getcart))) 0.75 "VTBlend_Linear" 0.0 false)
    (Default|TriggerStartDriving (Variables|Default|Getcart))
    (Variables|/Game/Core/General/BP_GameInstance.BP_GameInstance_C|SetcurrentGameState _asbp_game_instance "NewEnumerator0")))

(event Input|EnhancedActionEvents|EnhancedInputActionIA_DriveLeft
  (params (ActionValue :type Float%20%28double-precision%29) (ElapsedSeconds :type Float%20%28double-precision%29) (TriggeredSeconds :type Float%20%28double-precision%29) (InputAction :type Input%20Action%20Object%20Reference :default "/Game/Core/Input/IA_DriveLeft.IA_DriveLeft"))
  (bind _cart (Variables|Default|Getcart))
  (bind _cart_2 (Variables|Default|Getcart))
  (bind _cart_3 (Variables|Default|Getcart))
  (bind _cart_4 (Variables|Default|Getcart))
  (bind _asbp_game_instance (Utilities|Casting|CastToBP_GameInstance (Game|GetGameInstance)))
  (if (Utilities|Enum|Equal(Enum) (Variables|/Game/Core/General/BP_GameInstance.BP_GameInstance_C|GetcurrentGameState _asbp_game_instance) "NewEnumerator0")
    ;[1 1 1] Trigger Animation
    (if (and (== (Variables|/Game/Core/BP_Cart.BP_Cart_C|GetisChoosingPath _cart_4) false) (and (== (Variables|/Game/Core/BP_Cart.BP_Cart_C|GetisDriving _cart_4) true) (== (Variables|/Game/Core/BP_Cart.BP_Cart_C|GetisDrivingLeft _cart_4) false)))
      (Default|TriggerAnimLeft _cart_2)
      ;[0.4 0.95 0.3] WASD Controls
      ;;[0.4 0.95 0.3] Input Event Driving Left
      (if (== (Variables|/Game/Core/BP_Cart.BP_Cart_C|GetisDriving _cart_2) true)
        ;;;[1 1 1] isChangingLanes has to be false --> don't fire event multiple times
        (if (== (Variables|/Game/Core/BP_Cart.BP_Cart_C|GetisChangingLanes _cart_2) false)
          ;;;[1 1 1] Driving from right to middle --> driving left
          (if (and (== (Variables|/Game/Core/BP_Cart.BP_Cart_C|GetisDrivingLeft _cart_2) false) (== (Variables|/Game/Core/BP_Cart.BP_Cart_C|GetisDrivingRight _cart_2) true))
            (bind _newtrack_0 (Timeline|Timeline_FromRightToMiddle PlayFromStart)
              (:Update
                (Variables|/Game/Core/BP_Cart.BP_Cart_C|Setoffset _cart_3 (Math|Float|Lerp (* (* (Variables|Default|GetpathWidthModifier) -1.0) ActionValue) 0.0 _newtrack_0))
                (Variables|/Game/Core/BP_Cart.BP_Cart_C|SetisChangingLanes _cart_3 true))
              (:Finished
                (Variables|/Game/Core/BP_Cart.BP_Cart_C|SetisDrivingLeft _cart_3 false)
                (Variables|/Game/Core/BP_Cart.BP_Cart_C|SetisDrivingRight _cart_3 false)
                ;;;;[1 1 1 1 10] Cart can change lanes again --> events can be fired
                (Variables|/Game/Core/BP_Cart.BP_Cart_C|SetisChangingLanes _cart_3 false)))
            (else
              ;;;[1 1 1] Driving from middle to left --> driving left
              (if (and (== (Variables|/Game/Core/BP_Cart.BP_Cart_C|GetisDrivingLeft _cart_2) false) (== (Variables|/Game/Core/BP_Cart.BP_Cart_C|GetisDrivingRight _cart_2) false))
                (bind _newtrack_0_2 (Timeline|Timeline_FromMiddleToLeft PlayFromStart)
                  (:Update
                    (Variables|/Game/Core/BP_Cart.BP_Cart_C|Setoffset _cart (Math|Float|Lerp 0.0 (* ActionValue (Variables|Default|GetpathWidthModifier)) _newtrack_0_2))
                    (Variables|/Game/Core/BP_Cart.BP_Cart_C|SetisChangingLanes _cart true))
                  (:Finished
                    (Variables|/Game/Core/BP_Cart.BP_Cart_C|SetisDrivingLeft _cart true)
                    (Variables|/Game/Core/BP_Cart.BP_Cart_C|SetisDrivingRight _cart false)
                    (Variables|/Game/Core/BP_Cart.BP_Cart_C|SetisChangingLanes _cart false)))))))))))

(event EventBeginPlay
  (bind _timelinelength (Variables|Default|GettimelineLength))
  (Utilities|FlowControl|Sequence
    (:then_0
      ;[1 1 1] enable input system for cart
      (Input|AddMappingContext (PlayerController|LocalPlayerSubsystems|GetEnhancedInputLocalPlayerSubsystem (Game|GetPlayerController 0)) "/Game/Core/Input/IMC_Cart.IMC_Cart" 0 "(bIgnoreAllPressedKeysUntilRelease=True,bForceImmediately=False,bNotifyUserSettings=False)"))
    (:then_1
      ;[1 1 1] set variables
      (bind _asbp_game_instance (Utilities|Casting|CastToBP_GameInstance (Game|GetGameInstance)))
      (bind _cart (Default|GetCart _asbp_game_instance))
      (Variables|Default|Setcart _cart))
    (:then_2
      ;[1 1 1] Set play rates of timelines
      (Components|Timeline|SetPlayRate (Variables|Default|GetTimeline_FromRightToMiddle) _timelinelength)
      (Components|Timeline|SetPlayRate (Variables|Default|GetTimeline_FromLeftToRight) _timelinelength)
      (Components|Timeline|SetPlayRate (Variables|Default|GetTimeline_FromMiddleToRight) _timelinelength)
      (Components|Timeline|SetPlayRate (Variables|Default|GetTimeline_FromMiddleToLeft) _timelinelength))
    (:then_3
      ;[1 1 1] set spline movement reference
      (bind _asbp_game_instance_2 (Utilities|Casting|CastToBP_GameInstance (Game|GetGameInstance)))
      (bind _splinemovement (Default|GetSplineMovement _asbp_game_instance_2))
      (Variables|Default|SetsplineMovement _splinemovement))))

(fn ConstructionScript)