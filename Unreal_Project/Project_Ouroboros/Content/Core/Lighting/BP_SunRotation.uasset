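; Sun actor that moves a directional light through the day and hides it at night.
; On BeginPlay it registers itself with BP_GameInstance and restores the sun's visibility and pitch stored there.
; ChangeSunRotation checks the instance's day/night state, then either advances pitch by a fixed step or hides the light, updating its own IsSunHidden flag.
; NewDaySunPosition resets the pitch to the starting angle; a tick-counter-based rotation remains unused.
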(event Custom|Change%20SunRotation
  (bind _directionallight (Variables|Default|GetDirectionalLight))
  (bind _asbp_game_instance (Utilities|Casting|CastToBP_GameInstance (Game|GetGameInstance)))
  (bind _daynight (Default|GetDayNight _asbp_game_instance))
  (if (not (Variables|/Game/Core/Lighting/BP_DayNight.BP_DayNight_C|GetisNight _daynight))
    (Development|SetHiddeninGame _directionallight false false)
    (Variables|Default|SetisSunHidden false)
    (Transformation|SetActorRotation (Components|GetOwner _directionallight) (Math|Rotator|MakeRotator 0.0 (+ (.pitch (Transformation|GetActorRotation (Components|GetOwner (Variables|Default|GetDirectionalLight)))) 14.16) 0.0))
    (else
      (Development|SetHiddeninGame _directionallight true false)
      (Variables|Default|SetisSunHidden true))))

(event Custom|New%20Day%20Sun%20Position
  (Transformation|SetActorRotation (Components|GetOwner (Variables|Default|GetDirectionalLight)) (Math|Rotator|MakeRotator 0.0 -8e+01 0.0)))

(event EventBeginPlay
  (bind _asbp_game_instance (Utilities|Casting|CastToBP_GameInstance (Game|GetGameInstance)))
  (Default|SetSunRotation _asbp_game_instance self)
  (Development|SetHiddeninGame (Variables|Default|GetDirectionalLight) (Variables|/Game/Core/General/BP_GameInstance.BP_GameInstance_C|GetisSunHidden _asbp_game_instance) false)
  (Transformation|SetActorRotation (Math|Rotator|MakeRotator 0.0 (Variables|/Game/Core/General/BP_GameInstance.BP_GameInstance_C|GetsunYRotation _asbp_game_instance) 0.0)))

(fn ConstructionScript
  ;[1 0 0] geht irgendwie nicht im Construction Script? bei Begin Play gesetzt
)