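; BP_Fight is a turn-based fight manager that holds enemy and party lists and tracks turns, rounds and the acting side.
; On BeginPlay it derives round length from the combatant count, picks the starting side at random and starts the fight.
; BeginNextTurn increments Turn and copies it into RoundCounter, which SetNextRound increments on round boundaries.
; Attacks are only debug prints, and the acting side never switches after the start.
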(event Custom|Begin%20Next%20Turn
  (bind _result (Math|Integer|IncrementInt (Variables|Default|Getturn))
    (:%20%20
      (CallFunction|SetRoundCounter _result)
      (if (== (Variables|Default|GetisPartyFighting) true)
        ;[1 0 0] DEBUG
        (Development|PrintString "PLAYER ATTACK")
        (else
          ;[1 0 0] DEBUG
          (Development|PrintString "ENEMY ATTACK")))
      (CallFunction|SetNextRound))))

(event Custom|Start%20Fight
  (if (== (Variables|Default|GetisPartyFighting) true)
    ;[1 0 0] DEBUG
    (Development|PrintString "PLAYER ATTACK")
    (else
      ;[1 0 0] DEBUG
      (Development|PrintString "ENEMY ATTACK")))
  (CallFunction|SetNextRound))

(event EventBeginPlay
  (CallFunction|SetRoundCounter)
  (Variables|Default|Setturn 0)
  (CallFunction|CalculateRoundLength)
  (bind _ispartystarting (CallFunction|DecideStartingParty))
  (if _ispartystarting
    ;[1 0 0] Debug
    (Development|PrintString "Party Start")
    (CallFunction|SetIsPartyFighting true)
    (else
      (Development|PrintString "Enemies Start")
      (CallFunction|SetIsPartyFighting false)))
  (CallFunction|StartFight))

(fn ConstructionScript)

(fn GetIsPartyFighting
  (return (Variables|Default|GetisPartyFighting)))

(fn SetIsPartyFighting
  (params (isPartyFighting :type Boolean))
  (Variables|Default|SetisPartyFighting isPartyFighting)
  (return))

(fn GetRoundCounter
  (return (Variables|Default|GetroundCounter)))

(fn SetRoundCounter
  (params (roundCounter :type Integer))
  (Variables|Default|SetroundCounter roundCounter)
  (return))

(fn AddEnemy
  (params (newEnemy :type BP%20Base%20Enemy%20Object%20Reference))
  (Utilities|Array|Add (Variables|Default|Getenemies) newEnemy)
  (return))

(fn CalculateRoundLength
  (Variables|Default|SetroundLength (+ (Utilities|Array|Length (Variables|Default|Getenemies)) (Utilities|Array|Length (Variables|Default|GetpartyMembers))))
  (return))

(fn SetNextRound
  (if (== (Math|Integer|%(Integer) (Variables|Default|Getturn) (Variables|Default|GetroundLength)) 0)
    (bind _result (Math|Integer|IncrementInt (Variables|Default|GetroundCounter))
      (:%20%20
        (Variables|Default|SetroundCounter _result)
        (return)))))

(fn DecideStartingParty
  (if (== (Math|Integer|%(Integer) (Math|Random|RandomInteger 1000) 2) 0)
    (return true)
    (else
      (return false))))