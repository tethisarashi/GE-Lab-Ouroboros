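; BP_SunRotation is an actor that rotates a directional light to move the sun.
; Its construction script registers the actor with BP_GameInstance through SetSunRotation.
; The ChangeSunRotation event reads TickCounter from the game instance's tick manager and adds a local pitch scaled by that counter, so the rotation is relative rather than absolute.
; Nothing in this file calls that event, and Tick is unused.
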(event Custom|Change%20SunRotation
  (bind _asbp_game_instance (Utilities|Casting|CastToBP_GameInstance (Game|GetGameInstance)))
  (bind _tickmanager (Default|GetTickManager _asbp_game_instance))
  (Transformation|AddLocalRotation (Variables|Default|GetDirectionalLight) (Math|Rotator|MakeRotator 0.0 (* (Variables|/Game/Core/General/BP_TickManager.BP_TickManager_C|GettickCounter _tickmanager) 15.0) 0.0) false false))

(event EventBeginPlay)

(event Collision|EventActorBeginOverlap
  (params (OtherActor :type Actor%20Object%20Reference)))

(event EventTick
  (params (DeltaSeconds :type Float%20%28single-precision%29)))

(fn ConstructionScript
  (bind _asbp_game_instance (Utilities|Casting|CastToBP_GameInstance (Game|GetGameInstance)))
  (Default|SetSunRotation _asbp_game_instance self))