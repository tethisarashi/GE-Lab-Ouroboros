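; Spline movement controller that drives the player cart along the current spline and registers itself with the game instance.
; A timeline lerps distance along the spline to set cart position, lateral offset and tangent rotation, with play rate scaled by spline length for constant speed.
; At the end the cart chooses a path; splines tagged left and right are cached as options.
; Next-spline registration is an unfinished stub.
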(event Custom|Drive%20on%20Spline
  (bind _cart (Variables|Default|Getcart))
  (bind _cart_2 (Variables|Default|Getcart))
  ;[0.4 0.95 0.3] Move cart along spline
  (bind _newtrack_0 (Timeline|Timeline Play)
    (:Update
      (if (== (Variables|/Game/Core/BP_Cart.BP_Cart_C|GetisDriving _cart_2) true)
        ;;[1 1 1] set cart location on update
        (Transformation|SetActorLocation (Variables|Default|Getcart) (Spline|GetLocationatDistanceAlongSpline (Variables|Default|GetcurrentSpline) (Math|Float|Lerp 0.0 (Spline|GetDistanceAlongSplineatSplinePoint (Variables|Default|GetcurrentSpline) (- (Spline|GetNumberOfSplinePoints (Variables|Default|GetcurrentSpline)) 1)) _newtrack_0) "World") false false)
        (Transformation|AddActorLocalOffset _cart (Math|Vector|MakeVector 0.0 (Variables|/Game/Core/BP_Cart.BP_Cart_C|Getoffset _cart) 0.0) false false)
        ;;[1 1 1] set cart rotation on update
        (Transformation|SetActorRotation _cart (Math|Conversions|RotationFromXVector (Spline|GetTangentatDistanceAlongSpline (Variables|Default|GetcurrentSpline) (Math|Float|Lerp 0.0 (Spline|GetDistanceAlongSplineatSplinePoint (Variables|Default|GetcurrentSpline) (- (Spline|GetNumberOfSplinePoints (Variables|Default|GetcurrentSpline)) 1)) _newtrack_0) "World")))
        (Variables|Default|SetsplineLength (Math|Float|Lerp 0.0 (Spline|GetDistanceAlongSplineatSplinePoint (Variables|Default|GetcurrentSpline) (- (Spline|GetNumberOfSplinePoints (Variables|Default|GetcurrentSpline)) 1)) _newtrack_0))
        (else
          (Timeline|Timeline Stop))))
    (:Finished
      (Default|ChoosePath _cart_2))))

(event Custom|Drive%20on%20Chosen%20Spline
  (bind _cart (Variables|Default|Getcart))
  (bind _cart_2 (Variables|Default|Getcart))
  ;[0.4 0.95 0.3] Move cart along spline
  ;;[1 0.2108 0] register next spline
  (CallFunction|RegisterSplines)
  (bind _playrate (CallFunction|CalculatePlayrate))
  (Components|Timeline|SetPlayRate (Variables|Default|GetTimeline) _playrate)
  (bind _newtrack_0 (Timeline|Timeline PlayFromStart)
    (:Update
      (if (== (Variables|/Game/Core/BP_Cart.BP_Cart_C|GetisDriving _cart_2) true)
        ;;[1 1 1] set cart location on update
        (Transformation|SetActorLocation (Variables|Default|Getcart) (Spline|GetLocationatDistanceAlongSpline (Variables|Default|GetcurrentSpline) (Math|Float|Lerp 0.0 (Spline|GetDistanceAlongSplineatSplinePoint (Variables|Default|GetcurrentSpline) (- (Spline|GetNumberOfSplinePoints (Variables|Default|GetcurrentSpline)) 1)) _newtrack_0) "World") false false)
        (Transformation|AddActorLocalOffset _cart (Math|Vector|MakeVector 0.0 (Variables|/Game/Core/BP_Cart.BP_Cart_C|Getoffset _cart) 0.0) false false)
        ;;[1 1 1] set cart rotation on update
        (Transformation|SetActorRotation _cart (Math|Conversions|RotationFromXVector (Spline|GetTangentatDistanceAlongSpline (Variables|Default|GetcurrentSpline) (Math|Float|Lerp 0.0 (Spline|GetDistanceAlongSplineatSplinePoint (Variables|Default|GetcurrentSpline) (- (Spline|GetNumberOfSplinePoints (Variables|Default|GetcurrentSpline)) 1)) _newtrack_0) "World")))
        (Variables|Default|SetsplineLength (Math|Float|Lerp 0.0 (Spline|GetDistanceAlongSplineatSplinePoint (Variables|Default|GetcurrentSpline) (- (Spline|GetNumberOfSplinePoints (Variables|Default|GetcurrentSpline)) 1)) _newtrack_0))
        (else
          (Timeline|Timeline Stop))))
    (:Finished
      (Default|ChoosePath _cart_2))))

(event Custom|Register%20Splines
  ;[0.4 0.95 0.3] Register left and right spline for path choice
  (Utilities|FlowControl|Sequence
    (:then_0
      (bind _outactors (Actor|GetAllActorswithTag "left"))
      (for _array_element _outactors
        (Utilities|IsValid (Actor|GetComponentbyClass _array_element "/Script/Engine.SplineComponent")
          (:Is%20Valid
            (Variables|Default|SetsplineLeft (Actor|GetComponentbyClass _array_element "/Script/Engine.SplineComponent"))))))
    (:then_1
      (bind _outactors_2 (Actor|GetAllActorswithTag "right"))
      (for _array_element_2 _outactors_2
        (Utilities|IsValid (Actor|GetComponentbyClass _array_element_2 "/Script/Engine.SplineComponent")
          (:Is%20Valid
            (Variables|Default|SetsplineRight (Actor|GetComponentbyClass _array_element_2 "/Script/Engine.SplineComponent"))))))
    (:then_2
      ;;[1 0 0] DEBUG
      (Development|PrintString "Splines registriert"))))

(event Custom|Register%20Next%20Spline
  ;[1 0.2108 0] To Do: Register Splines for multiple Maps
  (bind _outactors (Actor|GetAllActorswithTag "next"))
  (for _array_element _outactors
    (Utilities|IsValid (Actor|GetComponentbyClass _array_element "/Script/Engine.SplineComponent"))))

(event Custom|Check%20Path
  ;[1 0.2108 0] To Do: Register Splines for multiple Maps
  (if (Components|ComponentHasTag (Variables|Default|GetcurrentSpline) "next")
    (Default|ChoosePath (Variables|Default|Getcart))
    (else
      (CallFunction|RegisterNextSpline))))

(event EventBeginPlay
  ;[0.4 0.95 0.3] Move cart along spline
  (CallFunction|RegisterSplines)
  (bind _asbp_game_instance (Utilities|Casting|CastToBP_GameInstance (Game|GetGameInstance)))
  (bind _cart (Default|GetCart _asbp_game_instance))
  (Variables|Default|Setcart _cart)
  ;;[1 1 1] Set play rate on begin play
  (bind _playrate (CallFunction|CalculatePlayrate))
  ;;;[1 1 1 1 12] The Play Rate of a timeline indicates the speed at which the timeline is played.
  (Components|Timeline|SetPlayRate (Variables|Default|GetTimeline) _playrate))

(event EventTick
  (params (DeltaSeconds :type Float%20%28single-precision%29))
  ;[1 1 1] Trigger driving event
  (if (Variables|/Game/Core/BP_Cart.BP_Cart_C|GetisDriving (Variables|Default|Getcart))
    (CallFunction|DriveonSpline)))

(fn ConstructionScript
  (bind _asbp_game_instance (Utilities|Casting|CastToBP_GameInstance (Game|GetGameInstance)))
  (Default|SetSplineMovement _asbp_game_instance self))

(fn CalculatePlayrate
  (return (/ 1e+01 (/ (Spline|GetSplineLength (Variables|Default|GetcurrentSpline)) (Variables|Default|GettimelineLength)))))