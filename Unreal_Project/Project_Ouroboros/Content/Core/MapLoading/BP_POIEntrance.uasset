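; BP_POIEntrance is a trigger actor that switches the game into a point-of-interest view when the cart enters it.
; On overlap with BP_Cart, it stops the cart driving and changes CurrentGameState on BP_GameInstance.
; It then calls MoveCameraToPOI on actors tagged "poicam", cast to BP_POICamera, and shows the mouse cursor.
; A direct view-target blend to the POI camera is present but unconnected.
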(event Collision|EventActorBeginOverlap
  (params (OtherActor :type Actor%20Object%20Reference))
  (bind _asbp_cart (Utilities|Casting|CastToBP_Cart OtherActor))
  (Default|TriggerStopDriving _asbp_cart)
  (bind _asbp_game_instance (Utilities|Casting|CastToBP_GameInstance (Game|GetGameInstance)))
  (Variables|/Game/Core/General/BP_GameInstance.BP_GameInstance_C|SetcurrentGameState _asbp_game_instance "NewEnumerator1")
  (bind _outactors (Actor|GetAllActorswithTag "poicam"))
  (for _array_element _outactors
    (bind _asbp_poicamera (Utilities|Casting|CastToBP_POICamera _array_element))
    (Default|MoveCameratoPOI _asbp_poicamera))
  (Variables|/Script/Engine.PlayerController|SetbShowMouseCursor (Game|GetPlayerController 0) true))

(fn ConstructionScript)