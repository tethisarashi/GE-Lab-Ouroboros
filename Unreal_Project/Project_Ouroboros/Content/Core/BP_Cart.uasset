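; BP_Cart is the party's cart, registered with the game instance, seating party members on mesh sockets.
; Starting or stopping driving runs or pauses the TickManager timer; path choice and a specific game state also stop it.
; Overlapping an unstarted BP_Fight stops and hides the cart and triggers the fight; afterwards it reappears, adding half the round count to the tick counter.
; It also handles camera blending, timed turn-animation flags and a physical-animation debug key.
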(event Custom|Trigger%20Start%20Driving
  (bind _tickmanager (Variables|Default|GettickManager))
  ;[0.4 0.95 0.3] Start/Stop driving
  (if (== (Variables|Default|GetisDriving) false)
    (Variables|Default|SetisDriving true)
    ;[0.4 0.95 0.3] Pause/Unpause Tick Timer
    (if (Variables|/Game/Core/General/BP_TickManager.BP_TickManager_C|GetisTimerPaused (Variables|Default|GettickManager))
      (Default|UnpauseTickTimer _tickmanager)
      (else
        (Default|StartTickTimer _tickmanager)))))

(event Custom|Trigger%20Stop%20Driving
  ;[0.4 0.95 0.3] Start/Stop driving
  (if (== (Variables|Default|GetisDriving) true)
    (Variables|Default|SetisDriving false)
    ;[0.4 0.95 0.3] Pause/Unpause Tick Timer
    (Default|PauseTickTimer (Variables|Default|GettickManager))))

(event Custom|Choose%20Path
  ;[0.4 0.95 0.3] Trigger path choice
  (CallFunction|TriggerStopDriving)
  (Variables|Default|SetisChoosingPath true))

(event Custom|Start%20Cartmode%20after%20Fight
  (bind _tickmanager (Variables|Default|GettickManager))
  ;[0.4 0.95 0.3] Set cart visibilty after fight
  (Rendering|SetActorHiddenInGame false)
  (Game|Player|SetViewTargetwithBlend (Game|GetPlayerController 0) (Components|GetOwner (Variables|Default|GetCamera)) 0.0 "VTBlend_Linear" 0.0 false)
  (Utilities|IsValid (stale Collision|EventActorBeginOverlap _asbp_fight)
    (:Is%20Valid
      (bind _roundcounter (Default|GetRoundCounter (stale Collision|EventActorBeginOverlap _asbp_fight)))
      (bind _output_get (Variables|/Game/Core/General/BP_TickManager.BP_TickManager_C|SettickCounter _tickmanager (+ (Variables|/Game/Core/General/BP_TickManager.BP_TickManager_C|GettickCounter _tickmanager) (/ _roundcounter 2))))
      (Development|PrintString (Utilities|String|ToString(Integer) _output_get)))))

(event Custom|Trigger_Anim_Left
  ;[1 1 1] Animation driving left/right
  (Variables|Default|SetisDrivingToLeft true)
  (Utilities|FlowControl|Delay 2.0)
  (Variables|Default|SetisDrivingToLeft false))

(event Custom|Trigger_Anim_Right
  ;[1 1 1] Animation driving left/right
  (Variables|Default|SetisDrivingToRight true)
  (Utilities|FlowControl|Delay 2.0)
  (Variables|Default|SetisDrivingToRight false))

(event Custom|MoveCameraToCart
  (bind _camera (Variables|Default|GetCamera))
  (bind _newtrack_0 (Timeline|Timeline Play)
    (:Update
      (Transformation|SetRelativeTransform _camera (Math|Transform|Lerp(Transform) (Transformation|GetRelativeTransform _camera) (Variables|Default|GetcartCamTransform) _newtrack_0) false false))))

(event Collision|EventActorBeginOverlap
  (params (OtherActor :type Actor%20Object%20Reference))
  ;[0.4 0.95 0.3] Trigger fight + set cart invisible
  (bind _asbp_fight (Utilities|Casting|CastToBP_Fight OtherActor))
  (bind _asbp_game_instance (Utilities|Casting|CastToBP_GameInstance (Game|GetGameInstance)))
  (Default|SetCurrentFight _asbp_game_instance _asbp_fight)
  (bind _isfightstarted (Default|GetIsFightStarted _asbp_fight))
  (if (not _isfightstarted)
    (Default|SetIsFightStarted _asbp_fight true)
    (CallFunction|TriggerStopDriving)
    (Rendering|SetActorHiddenInGame true)
    (Default|TriggerFight _asbp_fight)))

(event EventBeginPlay
  (bind _asbp_game_instance (Utilities|Casting|CastToBP_GameInstance (Game|GetGameInstance)))
  (bind _tickmanager (Default|GetTickManager _asbp_game_instance))
  (Variables|Default|SettickManager _tickmanager))

(event EventTick
  (params (DeltaSeconds :type Float%20%28single-precision%29))
  (bind _asbp_game_instance (Utilities|Casting|CastToBP_GameInstance (Game|GetGameInstance)))
  (if (Utilities|Enum|Equal(Enum) (Variables|/Game/Core/General/BP_GameInstance.BP_GameInstance_C|GetcurrentGameState _asbp_game_instance) "NewEnumerator5")
    (CallFunction|TriggerStopDriving)))

(event Input|KeyboardEvents|R
  (params (Key :type Key%20Structure :default "None"))
  ;[0.3005 0 0] Debug
  (:Pressed
    ;[1 1 1] activate physical animation
    (Default|TogglePhysicalAnimation (Variables|Default|GetBC_Cart_PhyAnim))))

(fn ConstructionScript
  (bind _asbp_game_instance (Utilities|Casting|CastToBP_GameInstance (Game|GetGameInstance)))
  (Default|SetCart _asbp_game_instance self))

(fn PlaceCharactersinCart
  (bind _asbp_game_instance (Utilities|Casting|CastToBP_GameInstance (Game|GetGameInstance)))
  (for (_array_element _array_index) (Variables|/Game/Core/Characters/BP_PartyMembers.BP_PartyMembers_C|GetpartyMembers (Variables|/Game/Core/General/BP_GameInstance.BP_GameInstance_C|GetpartyMembers _asbp_game_instance))
    (Transformation|AttachComponentToComponent _array_element (Variables|Default|GetSK_Entity_Cart) (Utilities|Array|Get(acopy) (Variables|Default|GetseatSockets) _array_index) "KeepRelative" "KeepRelative" "KeepRelative" true))
  (return))