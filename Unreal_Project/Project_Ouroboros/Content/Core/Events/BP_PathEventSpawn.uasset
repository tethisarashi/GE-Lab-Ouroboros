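; BP_PathEventSpawn is a placeholder actor that spawns one random path event, such as a fight, stone, loot or beggar.
; The construction script turns its PathEvents types into actor tags.
; On BeginPlay it picks an event and appearance at random, though Length-1 in RandomInteger excludes each array's last entry.
; It maps the type to a Blueprint class, spawns it with both choices passed in, then destroys itself.
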(event EventBeginPlay
  (bind _chosenevent (Private|ChooseEvent))
  (Variables|Private|SetchosenEvent (.eventtypes _chosenevent))
  (bind _chosenappearance (Private|ChooseAppearance (.possibleappearance _chosenevent)))
  (Variables|Private|SetchosenAppearance _chosenappearance)
  (bind _eventclass (CallFunction|ConvertEventTypetoClass (Variables|Private|GetchosenEvent)))
  (Game|SpawnActorfromClass _eventclass (Transformation|GetRelativeTransform (Variables|Default|GetTransform)) "Undefined" "MultiplyWithRoot" 0 (Variables|Private|GetchosenEvent) (Variables|Private|GetchosenAppearance) 0)
  (Actor|DestroyActor))

(event Collision|EventActorBeginOverlap
  (params (OtherActor :type Actor%20Object%20Reference)))

(event EventTick
  (params (DeltaSeconds :type Float%20%28single-precision%29)))

(fn ConstructionScript
  (for _array_element (Variables|Default|GetpathEvents)
    (if (!= (Utilities|String|StringToName (Utilities|String|EnumtoString (.eventtypes _array_element))) "E MAX")
      (Utilities|Array|Add (Variables|Default|GetpathEventTags) (Utilities|String|StringToName (Utilities|String|EnumtoString (.eventtypes _array_element))))))
  (Variables|Default|SetTags (Variables|Default|GetpathEventTags)))

(fn ChooseEvent
  (bind _pathevents (Variables|Default|GetpathEvents))
  (return (Utilities|Array|Get(acopy) _pathevents (Math|Random|RandomInteger (- (Utilities|Array|Length _pathevents) 1)))))

(fn ChooseAppearance
  (params (possibleAppearances :type Array%20of%20E_Appearance%20Enums :default "NewEnumerator0"))
  (return (Utilities|Array|Get(acopy) possibleAppearances (Math|Random|RandomInteger (- (Utilities|Array|Length possibleAppearances) 1)))))

(fn GetChosenEvent
  (return (Variables|Private|GetchosenEvent)))

(fn GetChosenAppearance
  (return (Variables|Private|GetchosenAppearance)))

(fn ConvertEventTypetoClass
  (params (eventType :type E_PathEvent%20Enum :default "NewEnumerator0"))
  (switch Utilities|FlowControl|Switch|SwitchonE_PathEvent eventType
    (:NewEnumerator0
      (Development|PrintString "KAMPF HALLO")
      (return "/Game/Core/Events/Fight/BP_Fight.BP_Fight_C"))
    (:NewEnumerator2
      (return "/Game/Core/Events/BP_Event_Stone.BP_Event_Stone_C"))
    (:NewEnumerator3
      (return "/Game/Core/Events/BP_Event_StoneFight.BP_Event_StoneFight_C"))
    (:NewEnumerator5
      (return "/Game/Core/Events/BP_Event_Loot.BP_Event_Loot_C"))
    (:NewEnumerator6
      (return "/Game/Core/Events/BP_Event_Beggar.BP_Event_Beggar_C"))))