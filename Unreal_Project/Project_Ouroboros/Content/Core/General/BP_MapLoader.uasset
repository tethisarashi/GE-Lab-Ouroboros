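; Map loader actor that saves game values when a BP_Cart overlaps it and can open the level TESTLEVEL.
; Its construction script registers it with BP_GameInstance through SetMapLoader, and the overlap calls SaveValues on that same game instance.
; LoadLevel opens the hardcoded level by name and is not called within this Blueprint, so it relies on an outside trigger.
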(event Custom|LoadLevel
  (Game|OpenLevel(byName) "TESTLEVEL"))

(event Collision|EventActorBeginOverlap
  (params (OtherActor :type Actor%20Object%20Reference))
  (Utilities|Casting|CastToBP_Cart OtherActor)
  (bind _asbp_game_instance (Utilities|Casting|CastToBP_GameInstance (Game|GetGameInstance)))
  (Default|SaveValues _asbp_game_instance))

(fn ConstructionScript
  (bind _asbp_game_instance (Utilities|Casting|CastToBP_GameInstance (Game|GetGameInstance)))
  (Default|SetMapLoader _asbp_game_instance self))