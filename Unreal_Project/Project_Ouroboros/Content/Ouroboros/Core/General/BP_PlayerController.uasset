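; Player controller that forwards Enhanced Input actions for driving to the level's BP_Cart.
; On BeginPlay it adds the cart mapping context, caches the cart and scales the timeline's play rate by its configured length.
; Start and stop actions call the cart's triggers, while left/right input writes its steering value directly.
; Canceled or completed steering plays a timeline that lerps that value toward zero, printing X for debugging.
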(event Input|EnhancedActionEvents|EnhancedInputActionIA_StartDriving
  (params (ActionValue :type Boolean) (ElapsedSeconds :type Float%20%28double-precision%29) (TriggeredSeconds :type Float%20%28double-precision%29) (InputAction :type Input%20Action%20Object%20Reference :default "/Game/Ouroboros/Core/Input/IA_StartDriving.IA_StartDriving"))
  ;[1 1 1] Input Events --> triggered in cart
  (Default|TriggerStartDriving (Variables|Default|Getcart)))

(event Input|EnhancedActionEvents|EnhancedInputActionIA_StopDriving
  (params (ActionValue :type Boolean) (ElapsedSeconds :type Float%20%28double-precision%29) (TriggeredSeconds :type Float%20%28double-precision%29) (InputAction :type Input%20Action%20Object%20Reference :default "/Game/Ouroboros/Core/Input/IA_StopDriving.IA_StopDriving"))
  ;[1 1 1] Input Events --> triggered in cart
  (Default|TriggerStopDriving (Variables|Default|Getcart)))

(event Input|EnhancedActionEvents|EnhancedInputActionIA_DriveLeftRight
  (params (ActionValue :type Vector%202D%20Structure) (ElapsedSeconds :type Float%20%28double-precision%29) (TriggeredSeconds :type Float%20%28double-precision%29) (InputAction :type Input%20Action%20Object%20Reference :default "/Game/Ouroboros/Core/Input/IA_DriveLeftRight.IA_DriveLeftRight"))
  (bind _cart (Variables|Default|Getcart))
  (:Triggered
    (Variables|/Game/Ouroboros/Core/BP_Cart.BP_Cart_C|SetactionValueLR _cart ActionValue))
  (:Canceled
    (bind _newtrack_0 (Timeline|Timeline Play)
      (:Update
        (Variables|/Game/Ouroboros/Core/BP_Cart.BP_Cart_C|SetactionValueLR _cart (Math|Vector2D|MakeVector2D (Math|Float|Lerp (.x (Variables|/Game/Ouroboros/Core/BP_Cart.BP_Cart_C|GetactionValueLR _cart)) 0.0 _newtrack_0) (Math|Float|Lerp (.y (Variables|/Game/Ouroboros/Core/BP_Cart.BP_Cart_C|GetactionValueLR _cart)) 0.0 _newtrack_0)))
        (Development|PrintString (Utilities|String|ToString(Float) (Math|Float|Lerp (.x (Variables|/Game/Ouroboros/Core/BP_Cart.BP_Cart_C|GetactionValueLR _cart)) 0.0 _newtrack_0))))))
  (:Completed
    (Timeline|Timeline Play)))

(event EventBeginPlay
  (Utilities|FlowControl|Sequence
    (:then_0
      ;[1 1 1] enable input system for cart
      (Input|AddMappingContext (PlayerController|LocalPlayerSubsystems|GetEnhancedInputLocalPlayerSubsystem (Game|GetPlayerController 0)) "/Game/Ouroboros/Core/Input/IMC_Cart.IMC_Cart" 0 "(bIgnoreAllPressedKeysUntilRelease=True,bForceImmediately=False,bNotifyUserSettings=False)"))
    (:then_1
      ;[1 1 1] set variables
      (bind _returnvalue (Actor|GetActorOfClass "/Game/Ouroboros/Core/BP_Cart.BP_Cart_C"))
      (Variables|Default|Setcart _returnvalue))
    (:then_2
      (Components|Timeline|SetPlayRate (Variables|Default|GetTimeline) (/ 1.0 (Variables|Default|GettimelineLength))))))

(fn ConstructionScript)