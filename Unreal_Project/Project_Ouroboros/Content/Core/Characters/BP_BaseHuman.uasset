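; BP_BaseHuman is a base Blueprint for human characters that exposes core survival and combat state.
; Simple getter functions return Health, Food, Defense and the current weapon.
; Only the weapon has a setter, backed by a variable whose TBD suffix suggests a placeholder.
; The event graph and construction script are empty, so no gameplay logic runs here yet.
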(event EventBeginPlay)

(event Collision|EventActorBeginOverlap
  (params (OtherActor :type Actor%20Object%20Reference)))

(event EventTick
  (params (DeltaSeconds :type Float%20%28single-precision%29)))

(fn ConstructionScript)

(fn GetHealth
  (return (Variables|Default|Gethealth)))

(fn GetFood
  (return (Variables|Default|Getfood)))

(fn GetDefense
  (return (Variables|Default|Getdefense)))

(fn GetCurrentWeapon
  (return (Variables|Default|GetcurrentWeaponTBD)))

(fn SetCurrentWeapon
  (params (newWeapon :type String))
  (Variables|Default|SetcurrentWeaponTBD newWeapon)
  (return))