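; BP_PartyMembers creates and holds the player's party of four characters: Bandit, Merchant, Peasant and Magician.
; Its construction script registers it with BP_GameInstance, and it exposes the party array through a getter.
; On BeginPlay it spawns each member below the world origin, out of view, and adds it to the array.
; A debug helper also gives each member a newly spawned base weapon.
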(event EventBeginPlay
  (bind _returnvalue (Math|Transform|MakeTransform "0.000000,0.000000,-250.000000"))
  (Utilities|FlowControl|Sequence
    (:then_0
      (bind _returnvalue_2 (Game|SpawnActorfromClass "/Game/Core/Characters/BP_BaseCharacter_Bandit.BP_BaseCharacter_Bandit_C" _returnvalue "Undefined" "MultiplyWithRoot" 0 0))
      (CallFunction|AddtoPartyMembers _returnvalue_2)
      ;[1 0 0] DEBUG
      (CallFunction|DEBUGAddWeapontoPlayer _returnvalue_2))
    (:then_1
      (bind _returnvalue_3 (Game|SpawnActorfromClass "/Game/Core/Characters/BP_BaseCharacter_Merchant.BP_BaseCharacter_Merchant_C" _returnvalue "Undefined" "MultiplyWithRoot" 0 0))
      (CallFunction|AddtoPartyMembers _returnvalue_3)
      (CallFunction|DEBUGAddWeapontoPlayer _returnvalue_3))
    (:then_2
      (bind _returnvalue_4 (Game|SpawnActorfromClass "/Game/Core/Characters/BP_BaseCharacter_Peasant.BP_BaseCharacter_Peasant_C" _returnvalue "Undefined" "MultiplyWithRoot" 0 0))
      (CallFunction|AddtoPartyMembers _returnvalue_4)
      (CallFunction|DEBUGAddWeapontoPlayer _returnvalue_4))
    (:then_3
      (bind _returnvalue_5 (Game|SpawnActorfromClass "/Game/Core/Characters/BP_BaseCharacter_Magician.BP_BaseCharacter_Magician_C" _returnvalue "Undefined" "MultiplyWithRoot" 0 0))
      (CallFunction|AddtoPartyMembers _returnvalue_5)
      (CallFunction|DEBUGAddWeapontoPlayer _returnvalue_5))))

(fn ConstructionScript
  (bind _asbp_game_instance (Utilities|Casting|CastToBP_GameInstance (Game|GetGameInstance)))
  (Default|SetPartyMembers _asbp_game_instance self))

(fn AddtoPartyMembers
  (params (newPartyMember :type BP%20Base%20Character%20Object%20Reference))
  (Utilities|Array|Add (Variables|Default|GetpartyMembers) newPartyMember)
  (return))

(fn GetPartyMembers
  (return (Variables|Default|GetpartyMembers)))

(fn DEBUGAddWeapontoPlayer
  (params (partyMember :type BP%20Base%20Character%20Object%20Reference))
  (bind _returnvalue (Game|SpawnActorfromClass "/Game/Core/Fight/BP_BaseWeapon.BP_BaseWeapon_C" (Math|Transform|MakeTransform "0, 0, 0") "Undefined" "MultiplyWithRoot" 0 0))
  (Default|SetCurrentWeapon partyMember _returnvalue)
  (return))