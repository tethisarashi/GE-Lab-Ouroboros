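; BP_SoundManager is a sound manager actor that provides one-call functions for UI, inventory, quest, item and combat sound effects.
; On BeginPlay it registers itself with BP_GameInstance so that it can be reached from there.
; Each function plays a fixed, non-spatialized 2D sound.
; Tick also casts to the game instance every frame and calls its PlayMusic whenever the Music reference is not valid, keeping music running.
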(event EventTick
  (params (DeltaSeconds :type Float%20%28single-precision%29))
  (bind _asbp_game_instance (Utilities|Casting|CastToBP_GameInstance (Game|GetGameInstance)))
  (Utilities|IsValid (Variables|/Game/Core/General/BP_GameInstance.BP_GameInstance_C|Getmusic _asbp_game_instance)
    (:Is%20Not%20Valid
      (Default|PlayMusic _asbp_game_instance))))

(event EventBeginPlay
  (bind _asbp_game_instance (Utilities|Casting|CastToBP_GameInstance (Game|GetGameInstance)))
  (Default|SetSoundManager _asbp_game_instance self))

(fn ConstructionScript)

(fn PlayButtonClickSound
  (Audio|PlaySound2D "/Game/Sound/Soundfiles/button_click_1.button_click_1" 1.0 1.0 0.0 0 0))

(fn PlayBanditDamageSound
  (Audio|PlaySound2D "/Game/Sound/Soundfiles/bandit_2_damage_2.bandit_2_damage_2" 1.0 1.0 0.0 0 0))

(fn PlayCharDamageSound
  (Audio|PlaySound2D "/Game/Sound/Soundfiles/bandit_damage_2.bandit_damage_2" 1.0 1.0 0.0 0 0))

(fn PlayOpenInventorySound
  (Audio|PlaySound2D "/Game/Sound/Soundfiles/inventar_öffnen_1.inventar_öffnen_1" 1.0 1.0 0.0 0 0))

(fn PlayCloseInventorySound
  (Audio|PlaySound2D "/Game/Sound/Soundfiles/inventar_schließen_1.inventar_schließen_1" 1.0 1.0 0.0 0 0))

(fn PlayQuestSound
  (Audio|PlaySound2D "/Game/Sound/Soundfiles/quest_notification.quest_notification" 1.0 1.0 0.0 0 0))

(fn PlayLootSound
  (Audio|PlaySound2D "/Game/Sound/Soundfiles/quest_annehmen.quest_annehmen" 1.0 1.0 0.0 0 0))

(fn PlayHealingSound
  (Audio|PlaySound2D "/Game/Sound/Soundfiles/healing_v2.healing_v2" 1.0 1.0 0.0 0 0))

(fn PlayFoodSound
  (Audio|PlaySound2D "/Game/Sound/Soundfiles/drink_2.drink_2" 1.0 1.0 0.0 0 0))

(fn PlayWeaponEquipSound
  (Audio|PlaySound2D "/Game/Sound/Soundfiles/item_equip_1.item_equip_1" 1.0 1.0 0.0 0 0))

(fn PlayPickUpSound
  (Audio|PlaySound2D "/Game/Sound/Soundfiles/pick_up_1.pick_up_1" 1.0 1.0 0.0 0 0))

(fn PlayDropSound
  (Audio|PlaySound2D "/Game/Sound/Soundfiles/pick_up_2.pick_up_2" 1.0 1.0 0.0 0 0))

(fn PlayScrollSound
  (Audio|PlaySound2D "/Game/Sound/Soundfiles/pick_up_3.pick_up_3" 1.0 1.0 0.0 0 0))

(fn PlayCharDeathSound
  (Audio|PlaySound2D "/Game/Sound/Soundfiles/bandit_death_1.bandit_death_1" 1.0 1.0 0.0 0 0))

(fn PlayBanditDeathSound
  (Audio|PlaySound2D "/Game/Sound/Soundfiles/bandit_2_death_1.bandit_2_death_1" 1.0 1.0 0.0 0 0))

(fn PlayAttackSound
  (Audio|PlaySound2D "/Game/Sound/Soundfiles/woosh_1.woosh_1" 1.0 1.0 0.0 0 0))