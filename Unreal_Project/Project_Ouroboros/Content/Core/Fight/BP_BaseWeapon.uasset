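; Base weapon Blueprint for the fight system, with placeholder base and special attacks that only print debug text.
; It stores special-attack state (max uses, use counter, last use and attack interval) behind getters and setters.
; Helpers increment the counter, report whether uses remain by testing equality with the max, and reset counter and last use.
; Nothing here enforces the limit or interval, and the event graph is empty.
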(event EventBeginPlay)

(event Collision|EventActorBeginOverlap
  (params (OtherActor :type Actor%20Object%20Reference)))

(event EventTick
  (params (DeltaSeconds :type Float%20%28single-precision%29)))

(fn ConstructionScript)

(fn BaseAttack
  (Development|PrintString "Base Attack")
  (return))

(fn SpecialAttack
  (Development|PrintString "SPECIAL ATTACK")
  (return))

(fn GetMaxUsesSpecialAttack
  (return (Variables|Default|GetmaxUsesSpecialAttack)))

(fn GetLastUseSpecialAttack
  (return (Variables|Default|GetlastUseSpecialAttack)))

(fn GetUseCounterSpecialAttack
  (return (Variables|Default|GetuseCounterSpecialAttack)))

(fn GetAttackIntervalSpecialAttack
  (return (Variables|Default|GetattackIntervalSpecialAttack)))

(fn SetAttackIntervalSpecialAttack
  (params (newAttackInterval :type Integer))
  (Variables|Default|SetattackIntervalSpecialAttack newAttackInterval)
  (return))

(fn SetMaxUsesSpecialAttack
  (params (newMaxUses :type Integer))
  (Variables|Default|SetmaxUsesSpecialAttack newMaxUses)
  (return))

(fn SetLastUseSpecialAttack
  (params (lastUse :type Integer))
  (Variables|Default|SetlastUseSpecialAttack lastUse)
  (return))

(fn SetUseCounterSpecialAttack
  (params (useCounter :type Integer))
  (Variables|Default|SetuseCounterSpecialAttack useCounter)
  (return))

(fn ResetWeaponValues
  (Variables|Default|SetlastUseSpecialAttack 0)
  (Variables|Default|SetuseCounterSpecialAttack 0)
  (return))

(fn IncreaseUseCounterSpecialAttack
  (bind _result (Math|Integer|IncrementInt (Variables|Default|GetuseCounterSpecialAttack))
    (:%20%20
      (Variables|Default|SetuseCounterSpecialAttack _result)
      (return))))

(fn CheckUsesLeftSpecialAttack
  (if (== (Variables|Default|GetuseCounterSpecialAttack) (Variables|Default|GetmaxUsesSpecialAttack))
    (return false)
    (else
      (return true))))