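; BP_DayNight tracks the day/night cycle while the cart is driving, registering itself with BP_GameInstance on construction.
; On Tick it reads the TickManager's counter, toggling IsNight every 12 game ticks, starting from day.
; A DoOnce, reset on multiples of 15, guards against repeated toggles within one game tick.
; Every 24 ticks it increments the day counter and briefly shows it in the WBP_DayNight widget.
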(event EventBeginPlay
  ;[1 1 1] Set isNight false at start of game
  (Variables|Default|SetisNight false)
  ;[1 1 1] set variables
  (bind _asbp_game_instance (Utilities|Casting|CastToBP_GameInstance (Game|GetGameInstance)))
  (bind _tickmanager (Default|GetTickManager _asbp_game_instance))
  (Variables|Default|SettickManager _tickmanager)
  (bind _cart (Default|GetCart _asbp_game_instance))
  (Variables|Default|Setcart _cart)
  (bind _returnvalue (UserInterface|CreateWidget "/Game/UI/WBP_DayNight.WBP_DayNight_C" (Game|GetPlayerController 0)))
  (bind _output_get (Variables|Default|Setui _returnvalue))
  (Widget|SetVisibility _output_get "Hidden")
  (UserInterface|Viewport|AddtoViewport _output_get 0))

(event EventTick
  (params (DeltaSeconds :type Float%20%28single-precision%29))
  (bind _ui (Variables|Default|Getui))
  (bind _tickmanager (Variables|Default|GettickManager))
  (bind _tickcounter (Variables|/Game/Core/General/BP_TickManager.BP_TickManager_C|GettickCounter _tickmanager))
  (if (Variables|/Game/Core/BP_Cart.BP_Cart_C|GetisDriving (Variables|Default|Getcart))
    (Utilities|FlowControl|Sequence
      (:then_0
        (if (>= (Variables|/Game/Core/General/BP_TickManager.BP_TickManager_C|GettickCounter (Variables|Default|GettickManager)) 2)
          ;[0.4 0.95 0.3] Night/day cycle --> night every %12 == 0 tick, day every %24 == 0 tick --> starting during day time
          (if (== (Math|Integer|%(Integer) _tickcounter 12) 0)
            ;;[1 1 1] change night/daytime only once every 12 ticks
            (Utilities|FlowControl|DoOnce false :!label _label
              (:Completed
                (Variables|Default|SetisNight (not (Variables|Default|GetisNight)))
                ;[0.4 0.95 0.3] increment day counter + set it in ui
                (if (== (Math|Integer|%(Integer) (Variables|/Game/Core/General/BP_TickManager.BP_TickManager_C|GettickCounter (Variables|Default|GettickManager)) 24) 0)
                  (bind _result (Math|Integer|IncrementInt (Variables|Default|GetdayCounter))
                    (:%20%20
                      (Variables|Default|SetdayCounter _result)
                      (Default|SetDayCounterText _ui (Utilities|Text|ToText(String) (Utilities|String|MakeLiteralString (Utilities|String|Append (Variables|Default|Getday) (Utilities|String|ToString(Integer) (Variables|Default|GetdayCounter))))))
                      (Widget|SetVisibility _ui "Visible")
                      (Utilities|FlowControl|Delay 1.5)
                      (Widget|SetVisibility _ui "Hidden")))))))))
      (:then_1
        ;;[1 1 1] reset do once node shortly after isNight got changed
        (if (== (Math|Integer|%(Integer) _tickcounter 15) 0)
          (goto _label Reset))))))

(fn ConstructionScript
  (bind _asbp_game_instance (Utilities|Casting|CastToBP_GameInstance (Game|GetGameInstance)))
  (Default|SetDayNight _asbp_game_instance self))