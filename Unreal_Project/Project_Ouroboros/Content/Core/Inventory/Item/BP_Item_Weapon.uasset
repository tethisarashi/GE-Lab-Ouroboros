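; BP_Item_Weapon is an inventory item Blueprint that holds a weapon's type and attack stats.
; Read-only getter functions expose the weapon type, base attack damage, and the special attack's damage, interval and maximum uses.
; The getters only return stored variables, with no attack or use-tracking logic in these graphs.
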(fn GetWeaponType
  (return (Variables|Default|GetweaponType)))

(fn GetAttackIntervalSpecialAttack
  (return (Variables|Default|GetattackIntervalSpecialAttack)))

(fn GetMaxUsesSpecialAttack
  (return (Variables|Default|GetmaxUsesSpecialAttack)))

(fn GetDamageBaseAttack
  (return (Variables|Default|GetdamageBaseAttack)))

(fn GetDamageSpecialAttack
  (return (Variables|Default|GetdamageSpecialAttack)))