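; Base roadside event actor that halts BP_Cart on overlap and calls StartEvent, which is an empty stub like FinishEvent.
; BeginPlay sets the visible or mystery-man mesh from ChosenAppearance.
; Any overlap sets a flag that makes Tick show the mouse cursor from then on.
; Reward helpers pick a random item type (food, heal, weapon, misc) and construct an item object from a random row of that type's DataTable.
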(event EventBeginPlay
  (CallFunction|SetAppearanceMesh))

(event Collision|EventActorBeginOverlap
  (params (OtherActor :type Actor%20Object%20Reference))
  (Development|PrintString (Utilities|GetDisplayName OtherActor))
  (Variables|Default|SetisOverlapped true)
  (bind _asbp_cart (Utilities|Casting|CastToBP_Cart OtherActor))
  (Default|TriggerStopDriving _asbp_cart)
  (CallFunction|StartEvent))

(event EventTick
  (params (DeltaSeconds :type Float%20%28single-precision%29))
  (if (Variables|Default|GetisOverlapped)
    (Variables|/Script/Engine.PlayerController|SetbShowMouseCursor (Game|GetPlayerController 0) true)))

(fn ConstructionScript)

(fn SetAppearanceMesh
  (switch Utilities|FlowControl|Switch|SwitchonE_Appearance (Variables|Private|GetchosenAppearance)
    (:NewEnumerator0
      (Components|SkeletalMesh|SetSkeletalMeshAsset (Variables|Default|GetSkeletalMesh) (Variables|Private|GetvisibleMesh)))
    (:NewEnumerator2
      (Components|SkeletalMesh|SetSkeletalMeshAsset (Variables|Default|GetSkeletalMesh) (Variables|Private|GetmysteryManMesh)))))

(fn StartEvent)

(fn ChooseRewardItemType
  (switch int (Math|Random|RandomInteger 4)
    (:Default
      _)
    (:0
      _)
    (:1
      (return "/Game/Core/Inventory/Item/BP_Item_Heal.BP_Item_Heal_C" "NewEnumerator1"))
    (:2
      (return "/Game/Core/Inventory/Item/BP_Item_Weapon.BP_Item_Weapon_C" "NewEnumerator0"))
    (:3
      (return "/Game/Core/Inventory/Item/BP_ItemObject.BP_ItemObject_C" "NewEnumerator3")))
  (return "/Game/Core/Inventory/Item/BP_Item_Food.BP_Item_Food_C" "NewEnumerator2"))

(fn CreateRewardItem
  (params (itemClass :type BP%20Item%20Object%20Class%20Reference) (itemType :type E_ItemType%20Enum :default "NewEnumerator0"))
  (switch Utilities|FlowControl|Switch|SwitchonE_ItemType itemType
    (:NewEnumerator0
      (bind _outrownames (DataTable|GetDataTableRowNames "/Game/Core/Inventory/Item/Datatables/DT_InventoryItemsWeapon.DT_InventoryItemsWeapon"))
      (bind _returnvalue (Utilities|GetDataTableRow "/Game/Core/Inventory/Item/Datatables/DT_InventoryItemsWeapon.DT_InventoryItemsWeapon" (Utilities|Array|Get(acopy) _outrownames (Math|Random|RandomInteger (- (Utilities|Array|Length _outrownames) 1))))
        (:then
          (bind _asbp_item_weapon (Utilities|Casting|CastToBP_Item_WeaponClass itemClass))
          (bind _returnvalue_2 (Game|ConstructObjectfromClass _asbp_item_weapon (.attackintervalspecialattack _returnvalue) (.maxusesspecialattack _returnvalue) (.weapontype _returnvalue) (.damagebaseattack _returnvalue) (.damagespecialattack _returnvalue) (.dimensions _returnvalue) (.icon _returnvalue) (.iconrotated _returnvalue) (.isrotated _returnvalue) (.type _returnvalue) (.itemname _returnvalue) (.itemid _returnvalue) (.merchantprice _returnvalue) (.playerprice _returnvalue) (.topleftindex _returnvalue) (.isstartitem _returnvalue) (.startamount _returnvalue)))
          (return _returnvalue_2))))
    (:NewEnumerator1
      (bind _outrownames_2 (DataTable|GetDataTableRowNames "/Game/Core/Inventory/Item/Datatables/DT_InventoryItemsHeal.DT_InventoryItemsHeal"))
      (bind _returnvalue_3 (Utilities|GetDataTableRow "/Game/Core/Inventory/Item/Datatables/DT_InventoryItemsHeal.DT_InventoryItemsHeal" (Utilities|Array|Get(acopy) _outrownames_2 (Math|Random|RandomInteger (- (Utilities|Array|Length _outrownames_2) 1))))
        (:then
          (bind _asbp_item_heal (Utilities|Casting|CastToBP_Item_HealClass itemClass))
          (bind _returnvalue_4 (Game|ConstructObjectfromClass _asbp_item_heal (.healvalue _returnvalue_3) (.dimensions _returnvalue_3) (.icon _returnvalue_3) (.iconrotated _returnvalue_3) (.isrotated _returnvalue_3) (.type _returnvalue_3) (.itemname _returnvalue_3) (.itemid _returnvalue_3) (.merchantprice _returnvalue_3) (.playerprice _returnvalue_3) (.topleftindex _returnvalue_3) (.isstartitem _returnvalue_3) (.startamount _returnvalue_3)))
          (return _returnvalue_4))))
    (:NewEnumerator2
      (bind _outrownames_3 (DataTable|GetDataTableRowNames "/Game/Core/Inventory/Item/Datatables/DT_InventoryItemsFood.DT_InventoryItemsFood"))
      (bind _returnvalue_5 (Utilities|GetDataTableRow "/Game/Core/Inventory/Item/Datatables/DT_InventoryItemsFood.DT_InventoryItemsFood" (Utilities|Array|Get(acopy) _outrownames_3 (Math|Random|RandomInteger (- (Utilities|Array|Length _outrownames_3) 1))))
        (:then
          (bind _asbp_item_food (Utilities|Casting|CastToBP_Item_FoodClass itemClass))
          (bind _returnvalue_6 (Game|ConstructObjectfromClass _asbp_item_food (.foodvalue _returnvalue_5) (.dimensions _returnvalue_5) (.icon _returnvalue_5) (.iconrotated _returnvalue_5) (.isrotated _returnvalue_5) (.type _returnvalue_5) (.itemname _returnvalue_5) (.itemid _returnvalue_5) (.merchantprice _returnvalue_5) (.playerprice _returnvalue_5) (.topleftindex _returnvalue_5) (.isstartitem _returnvalue_5) (.startamount _returnvalue_5)))
          (return _returnvalue_6))))
    (:NewEnumerator3
      (bind _outrownames_4 (DataTable|GetDataTableRowNames "/Game/Core/Inventory/Item/Datatables/DT_InventoryItemsMisc.DT_InventoryItemsMisc"))
      (bind _returnvalue_7 (Utilities|GetDataTableRow "/Game/Core/Inventory/Item/Datatables/DT_InventoryItemsMisc.DT_InventoryItemsMisc" (Utilities|Array|Get(acopy) _outrownames_4 (Math|Random|RandomInteger (- (Utilities|Array|Length _outrownames_4) 1))))
        (:then
          (bind _asbp_item_object (Utilities|Casting|CastToBP_ItemObjectClass itemClass))
          (bind _returnvalue_8 (Game|ConstructObjectfromClass _asbp_item_object (.dimensions _returnvalue_7) (.icon _returnvalue_7) (.iconrotated _returnvalue_7) (.isrotated _returnvalue_7) (.type _returnvalue_7) (.itemname _returnvalue_7) (.itemid _returnvalue_7) (.merchantprice _returnvalue_7) (.playerprice _returnvalue_7) (.topleftindex _returnvalue_7) (.isstartitem _returnvalue_7) (.startamount _returnvalue_7)))
          (return _returnvalue_8))))))

(fn FinishEvent)