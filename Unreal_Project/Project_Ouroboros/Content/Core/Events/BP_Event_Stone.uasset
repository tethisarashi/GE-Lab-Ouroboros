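; Stone road event actor that plays the cart's damage animation on overlap and, when the event starts, shows a repair choice widget with cursor and scroll sound.
; The kit option, enabled only if a "repair kit" is in the main inventory, consumes that item.
; Repairing by hand instead randomly advances the tick counter and sun rotation and drains each party member's food.
; Either choice closes the widget and destroys the actor.
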(event Custom|RepairByHand
  (CallFunction|Repair)
  (CallFunction|FinishEvent))

(event Custom|FinishStoneEvent
  (CallFunction|UseRepairSet)
  (CallFunction|FinishEvent))

(event EventBeginPlay
  (bind _returnvalue (UserInterface|CreateWidget "/Game/UI/Events/WBP_StoneEvent.WBP_StoneEvent_C" (Game|GetPlayerController 0)))
  (Variables|Default|Setui _returnvalue)
  (EventDispatchers|BindEventtoRepairbyHand (Variables|Default|Getui) (delegate Custom|RepairByHand))
  (EventDispatchers|BindEventtoFinishStoneEvent (Variables|Default|Getui) (delegate Custom|FinishStoneEvent)))

(event Collision|EventActorBeginOverlap
  (params (OtherActor :type Actor%20Object%20Reference))
  (|CallParentFunction OtherActor)
  (bind _asbp_game_instance (Utilities|Casting|CastToBP_GameInstance (Game|GetGameInstance)))
  (Default|TriggerAnimDamage (Default|GetAnimationBlueprint (Variables|/Game/Core/General/BP_GameInstance.BP_GameInstance_C|Getcart _asbp_game_instance))))

(event EventTick
  (params (DeltaSeconds :type Float%20%28single-precision%29))
  (|CallParentFunction DeltaSeconds) ; This node is disabled and will not be called.\nDrag off pins to build functionality.
)

(fn ConstructionScript
  (|CallParentFunction))

(fn StartEvent
  (bind _ui (Variables|Default|Getui))
  (|CallParentFunction)
  (UserInterface|Viewport|AddtoViewport (Variables|Default|Getui) 0)
  (bind _asbp_game_instance (Utilities|Casting|CastToBP_GameInstance (Game|GetGameInstance)))
  (Default|PlayScrollSound (Default|GetSoundManager _asbp_game_instance))
  (Variables|/Script/Engine.PlayerController|SetbShowMouseCursor (Game|GetPlayerController 0) true)
  (bind _isrepairsetfound (CallFunction|CheckRepairSet))
  (if _isrepairsetfound
    (Default|EnableRepairSetButton _ui)
    (else
      (Default|DisableRepairSetButton _ui))))

(fn FinishEvent
  (|CallParentFunction)
  (Widget|RemovefromParent (Variables|Default|Getui))
  (Variables|/Script/Engine.PlayerController|SetbShowMouseCursor (Game|GetPlayerController 0) false)
  (Actor|DestroyActor))

(fn CheckRepairSet
  (bind _asbp_game_instance (Utilities|Casting|CastToBP_GameInstance (Game|GetGameInstance)))
  (for _array_element (Default|GetIndividualItemObjects (Variables|/Game/Core/General/BP_GameInstance.BP_GameInstance_C|GetmainInventory _asbp_game_instance))
    (Utilities|IsValid _array_element
      (:Is%20Valid
        (if (== (Default|GetItemName _array_element) "repair kit")
          (Variables|Default|SetrepairSet _array_element)
          (return true)))))
  (return false))

(fn Repair
  (bind _returnvalue (Math|Random|RandomIntegerinRange 5 8))
  (bind _asbp_game_instance (Utilities|Casting|CastToBP_GameInstance (Game|GetGameInstance)))
  (bind _tickmanager (Default|GetTickManager _asbp_game_instance))
  (Default|UpdateTickCounterAfterEvent _tickmanager)
  (bind _output_get (Variables|/Game/Core/General/BP_TickManager.BP_TickManager_C|SettickCounter _tickmanager (+ (Variables|/Game/Core/General/BP_TickManager.BP_TickManager_C|GettickCounter _tickmanager) _returnvalue)))
  (Development|PrintString (Utilities|String|ToString(Integer) _output_get))
  (for _array_element (Variables|/Game/Core/Characters/BP_PartyMembers.BP_PartyMembers_C|GetpartyMembers (Variables|/Game/Core/General/BP_GameInstance.BP_GameInstance_C|GetpartyMembers _asbp_game_instance))
    (bind _food (Default|GetFood _array_element))
    (Default|SetFood _array_element (- _food (* _returnvalue 2))))
  (Default|SetSunRotation (Variables|/Game/Core/General/BP_GameInstance.BP_GameInstance_C|GetsunRotation _asbp_game_instance) _returnvalue))

(fn UseRepairSet
  (bind _asbp_game_instance (Utilities|Casting|CastToBP_GameInstance (Game|GetGameInstance)))
  (Default|RemoveItem (Variables|/Game/Core/General/BP_GameInstance.BP_GameInstance_C|GetmainInventory _asbp_game_instance) (Variables|Default|GetrepairSet)))