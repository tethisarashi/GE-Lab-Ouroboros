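; Spline-based road actor that builds its mesh in the Construction Script, one spline mesh per segment.
; Each segment follows the spline's positions and tangents, taking its width and height from point scale.
; All segments share one dynamic material instance fed by per-road falloff, dirt, tiling, noise and colour variables.
; Custom primitive data flags the first and last segments with opposite signs, likely for end falloff in the material.
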(event EventBeginPlay)

(event Collision|EventActorBeginOverlap
  (params (OtherActor :type Actor%20Object%20Reference)))

(event EventTick
  (params (DeltaSeconds :type Float%20%28single-precision%29)))

(fn ConstructionScript
  (bind _spline (Variables|Default|GetSpline))
  (bind _returnvalue (Rendering|Material|CreateDynamicMaterialInstance (Variables|Default|GetRoadMaterial) "None" "None" :!class /Script/Engine.KismetMaterialLibrary))
  (Variables|Default|SetRoadMaterialInstance _returnvalue)
  (for _index (range 0 (- (Spline|GetNumberOfSplinePoints (Variables|Default|GetSpline)) 2))
    (bind _returnvalue_2 (AddComponent|AddSplineMeshComponent false))
    (SplineMesh|SetForwardAxis _returnvalue_2 "X" true)
    (SplineMesh|SetStartandEnd _returnvalue_2 (Spline|GetLocationatSplinePoint _spline _index "Local") (Spline|GetTangentatSplinePoint _spline _index "Local") (Spline|GetLocationatSplinePoint _spline (+ _index 1) "Local") (Spline|GetTangentatSplinePoint _spline (+ _index 1) "Local") true :!class /Script/Engine.SplineMeshComponent)
    (SplineMesh|SetStartScale _returnvalue_2 (Math|Vector2D|MakeVector2D (.y (Spline|GetScaleatSplinePoint _spline _index)) (.z (Spline|GetScaleatSplinePoint _spline _index))) true :!class /Script/Engine.SplineMeshComponent)
    (SplineMesh|SetEndScale _returnvalue_2 (Math|Vector2D|MakeVector2D (.y (Spline|GetScaleatSplinePoint _spline (+ _index 1))) (.z (Spline|GetScaleatSplinePoint _spline (+ _index 1)))) true :!class /Script/Engine.SplineMeshComponent)
    (Rendering|Material|SetMaterial _returnvalue_2 0 (Variables|Default|GetRoadMaterialInstance))
    (if (== _index 0)
      (Rendering|Material|SetCustomPrimitiveDataFloat _returnvalue_2 0 1.0)
      (elif (== _index (- (Spline|GetNumberOfSplinePoints (Variables|Default|GetSpline)) 2))
        (Rendering|Material|SetCustomPrimitiveDataFloat _returnvalue_2 0 -1.0))))
  ;[1 1 1] Make all these variables Public so you can edit them in the editor PER road
  (Rendering|Material|SetScalarParameterValue (Variables|Default|GetRoadMaterialInstance) "RoadFalloffOffset" (Variables|Default|GetRoad%20Falloff%20Offset) :!class /Script/Engine.MaterialInstanceDynamic)
  (Rendering|Material|SetScalarParameterValue (Variables|Default|GetRoadMaterialInstance) "RoadFalloffHardness" (Variables|Default|GetRoad%20Falloff%20Hard) :!class /Script/Engine.MaterialInstanceDynamic)
  (Rendering|Material|SetScalarParameterValue (Variables|Default|GetRoadMaterialInstance) "RoadOpacityContrast" (Variables|Default|GetRoad%20Opacity%20Contrast) :!class /Script/Engine.MaterialInstanceDynamic)
  (Rendering|Material|SetScalarParameterValue (Variables|Default|GetRoadMaterialInstance) "NormalFlatness" (Variables|Default|GetRoad%20Normal%20Flatness) :!class /Script/Engine.MaterialInstanceDynamic)
  (Rendering|Material|SetScalarParameterValue (Variables|Default|GetRoadMaterialInstance) "DirtOffset" (Variables|Default|GetDirtOffset) :!class /Script/Engine.MaterialInstanceDynamic)
  (Rendering|Material|SetScalarParameterValue (Variables|Default|GetRoadMaterialInstance) "DirtContrast" (Variables|Default|GetDirtContrast) :!class /Script/Engine.MaterialInstanceDynamic)
  (Rendering|Material|SetScalarParameterValue (Variables|Default|GetRoadMaterialInstance) "Tiling X" (Variables|Default|GetTiling%20X) :!class /Script/Engine.MaterialInstanceDynamic)
  (Rendering|Material|SetScalarParameterValue (Variables|Default|GetRoadMaterialInstance) "Tiling Y" (Variables|Default|GetTiling%20Y) :!class /Script/Engine.MaterialInstanceDynamic)
  (Rendering|Material|SetScalarParameterValue (Variables|Default|GetRoadMaterialInstance) "NoiseInfluence" (Variables|Default|GetNoiseInfluence) :!class /Script/Engine.MaterialInstanceDynamic)
  (Rendering|Material|SetVectorParameterValue (Variables|Default|GetRoadMaterialInstance) "DirtColour" (Variables|Default|GetDirtColour) :!class /Script/Engine.MaterialInstanceDynamic)
  (Rendering|Material|SetVectorParameterValue (Variables|Default|GetRoadMaterialInstance) "RoadColour" (Variables|Default|GetRoadColour) :!class /Script/Engine.MaterialInstanceDynamic)
  (Rendering|Material|SetScalarParameterValue (Variables|Default|GetRoadMaterialInstance) "RoadEndFalloffHardness" (Variables|Default|GetRoadEndFalloffHardness) :!class /Script/Engine.MaterialInstanceDynamic))