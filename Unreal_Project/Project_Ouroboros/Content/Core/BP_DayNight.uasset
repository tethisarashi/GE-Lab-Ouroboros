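; BP_DayNight tracks the day/night cycle as an IsNight flag, starting in daytime.
; On BeginPlay it finds the BP_TickManager and BP_Cart actors.
; While the cart is driving, Tick polls the manager's TickCounter and flips IsNight on multiples of 12, skipping the initial count.
; A DoOnce guards against repeated flips and re-arms on multiples of 15, which coincide with flip counts every 60.
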(event EventBeginPlay
  ;[1 1 1] Set isNight false at start of game
  (Variables|Default|SetisNight false)
  ;[1 1 1] set variables
  (bind _returnvalue (Actor|GetActorOfClass "/Game/Core/General/BP_TickManager.BP_TickManager_C"))
  (Variables|Default|SettickManager _returnvalue)
  (bind _returnvalue_2 (Actor|GetActorOfClass "/Game/Core/BP_Cart.BP_Cart_C"))
  (Variables|Default|Setcart _returnvalue_2))

(event EventTick
  (params (DeltaSeconds :type Float%20%28single-precision%29))
  (bind _tickmanager (Variables|Default|GettickManager))
  (bind _tickcounter (Variables|/Game/Core/General/BP_TickManager.BP_TickManager_C|GettickCounter _tickmanager))
  (if (Variables|/Game/Core/BP_Cart.BP_Cart_C|GetisDriving (Variables|Default|Getcart))
    (Utilities|FlowControl|Sequence
      (:then_0
        (if (>= (Variables|/Game/Core/General/BP_TickManager.BP_TickManager_C|GettickCounter (Variables|Default|GettickManager)) 2)
          ;[0.4 0.95 0.3] Night/day cycle --> night every %12 == 0 tick, day every %24 == 0 tick --> starting during day time
          (if (== (Math|Integer|%(Integer) _tickcounter 12) 0)
            ;;[1 1 1] change night/daytime only once every 12 ticks
            (Utilities|FlowControl|DoOnce false :!label _label
              (:Completed
                (Variables|Default|SetisNight (not (Variables|Default|GetisNight))))))))
      (:then_1
        ;;[1 1 1] reset do once node shortly after isNight got changed
        (if (== (Math|Integer|%(Integer) _tickcounter 15) 0)
          (goto _label Reset))))))

(fn ConstructionScript)