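; Spline movement actor that drives a referenced Cart actor along its spline, placing it at the first spline point on construction.
; On BeginPlay it sets the timeline play rate to the inverse of TimelineLength and starts playback.
; Each update maps timeline alpha to distance along the spline, setting cart location and tangent-based rotation.
; On finish it calls play again as a debug stand-in for switching to a new spline.
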(event Custom|PlayTimeline
  (bind _spline (Variables|Default|GetSpline))
  (bind _spline_2 (Variables|Default|GetSpline))
  (bind _cart (Variables|Default|Getcart))
  ;[0.4 0.95 0.3] Move cart along spline
  (bind _newtrack_0 (Timeline|Timeline Play)
    (:Update
      ;;[1 1 1] set cart location on update
      (Transformation|SetActorLocation _cart (Spline|GetLocationatDistanceAlongSpline _spline_2 (Math|Float|Lerp 0.0 (Spline|GetDistanceAlongSplineatSplinePoint _spline (- (Spline|GetNumberOfSplinePoints _spline) 1)) _newtrack_0) "World") false false)
      ;;[1 1 1] set cart rotation on update
      (Transformation|SetActorRotation _cart (Math|Conversions|RotationFromXVector (Spline|GetTangentatDistanceAlongSpline _spline_2 (Math|Float|Lerp 0.0 (Spline|GetDistanceAlongSplineatSplinePoint _spline (- (Spline|GetNumberOfSplinePoints _spline) 1)) _newtrack_0) "World")))
      (Variables|Default|SetsplineLength (Math|Float|Lerp 0.0 (Spline|GetDistanceAlongSplineatSplinePoint _spline (- (Spline|GetNumberOfSplinePoints _spline) 1)) _newtrack_0)))
    (:Finished
      ;;[1 0 0] Debug
      ;; --> should move to new spline when timeline iis finished --> restarts timeline atm
      (CallFunction|PlayTimeline))))

(event EventBeginPlay
  ;[0.4 0.95 0.3] Move cart along spline
  ;;[1 1 1] Trigger timeline event that starts spline drive on begin play
  ;;;[1 1 1 1 12] The Play Rate of a timeline indicates the speed at which the timeline is played.
  (Components|Timeline|SetPlayRate (Variables|Default|GetTimeline) (/ 1.0 (Variables|Default|GettimelineLength)))
  (CallFunction|PlayTimeline))

(fn ConstructionScript
  ;[1 1 1] set cart start point to point on spline with index zero on construction
  (Transformation|SetActorLocation (Variables|Default|Getcart) (Spline|GetLocationatSplinePoint (Variables|Default|GetSpline) 0 "World") false false))