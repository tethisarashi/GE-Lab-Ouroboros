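; Level exit actor that saves game values and shows a load-level widget when BP_Cart overlaps it.
; It creates the hidden widget on BeginPlay and registers itself with BP_GameInstance in its construction script.
; The LoadLevel event reads the instance's StageCounter, randomly picks one of that stage's three map pools (regular, City, POI), then opens a random map from it.
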(event Custom|LoadLevel
  (bind _returnvalue (Math|Random|RandomIntegerinRange 0 2))
  (bind _asbp_game_instance (Utilities|Casting|CastToBP_GameInstance (Game|GetGameInstance)))
  (switch int (Variables|/Game/Core/General/BP_GameInstance.BP_GameInstance_C|GetstageCounter _asbp_game_instance)
    (:1
      (bind _mapname (CallFunction|GetRandomMapStage1 _returnvalue))
      (Game|OpenLevel(byName) _mapname))
    (:2
      (bind _mapname_2 (CallFunction|GetRandomMapStage2 _returnvalue))
      (Game|OpenLevel(byName) _mapname_2))
    (:3
      (bind _mapname_3 (CallFunction|GetRandomMapStage3 _returnvalue))
      (Game|OpenLevel(byName) _mapname_3))))

(event EventBeginPlay
  (bind _returnvalue (UserInterface|CreateWidget "/Game/UI/WBP_LoadLevel.WBP_LoadLevel_C" (Game|GetPlayerController 0)))
  (bind _output_get (Variables|Default|Setui _returnvalue))
  (UserInterface|Viewport|AddtoViewport _output_get 0)
  (Widget|SetVisibility _output_get "Hidden"))

(event Collision|EventActorBeginOverlap
  (params (OtherActor :type Actor%20Object%20Reference))
  (Utilities|Casting|CastToBP_Cart OtherActor)
  (Widget|SetVisibility (Variables|Default|Getui) "Visible")
  (bind _asbp_game_instance (Utilities|Casting|CastToBP_GameInstance (Game|GetGameInstance)))
  (Default|SaveValues _asbp_game_instance))

(fn ConstructionScript
  (bind _asbp_game_instance (Utilities|Casting|CastToBP_GameInstance (Game|GetGameInstance)))
  (Default|SetMapLoader _asbp_game_instance self))

(fn GetRandomMapStage1
  (params (type :type Integer))
  (bind _asbp_game_instance (Utilities|Casting|CastToBP_GameInstance (Game|GetGameInstance)))
  (switch int type
    (:0
      (return (Utilities|Array|Get(acopy) (Variables|/Game/Core/General/BP_GameInstance.BP_GameInstance_C|GetmapNamesStage1 _asbp_game_instance) (Math|Random|RandomIntegerinRange 0 (- (Utilities|Array|Length (Variables|/Game/Core/General/BP_GameInstance.BP_GameInstance_C|GetmapNamesStage1 _asbp_game_instance)) 1)))))
    (:1
      (return (Utilities|Array|Get(acopy) (Variables|/Game/Core/General/BP_GameInstance.BP_GameInstance_C|GetmapNamesStage1_City _asbp_game_instance) (Math|Random|RandomIntegerinRange 0 (- (Utilities|Array|Length (Variables|/Game/Core/General/BP_GameInstance.BP_GameInstance_C|GetmapNamesStage1_City _asbp_game_instance)) 1)))))
    (:2
      (return (Utilities|Array|Get(acopy) (Variables|/Game/Core/General/BP_GameInstance.BP_GameInstance_C|GetmapNamesStage1_POI _asbp_game_instance) (Math|Random|RandomIntegerinRange 0 (- (Utilities|Array|Length (Variables|/Game/Core/General/BP_GameInstance.BP_GameInstance_C|GetmapNamesStage1_POI _asbp_game_instance)) 1)))))))

(fn GetRandomMapStage2
  (params (type :type Integer))
  (bind _asbp_game_instance (Utilities|Casting|CastToBP_GameInstance (Game|GetGameInstance)))
  (switch int type
    (:0
      (return (Utilities|Array|Get(acopy) (Variables|/Game/Core/General/BP_GameInstance.BP_GameInstance_C|GetmapNamesStage2 _asbp_game_instance) (Math|Random|RandomIntegerinRange 0 (- (Utilities|Array|Length (Variables|/Game/Core/General/BP_GameInstance.BP_GameInstance_C|GetmapNamesStage2 _asbp_game_instance)) 1)))))
    (:1
      (return (Utilities|Array|Get(acopy) (Variables|/Game/Core/General/BP_GameInstance.BP_GameInstance_C|GetmapNamesStage2_City _asbp_game_instance) (Math|Random|RandomIntegerinRange 0 (- (Utilities|Array|Length (Variables|/Game/Core/General/BP_GameInstance.BP_GameInstance_C|GetmapNamesStage2_City _asbp_game_instance)) 1)))))
    (:2
      (return (Utilities|Array|Get(acopy) (Variables|/Game/Core/General/BP_GameInstance.BP_GameInstance_C|GetmapNamesStage2_POI _asbp_game_instance) (Math|Random|RandomIntegerinRange 0 (- (Utilities|Array|Length (Variables|/Game/Core/General/BP_GameInstance.BP_GameInstance_C|GetmapNamesStage2_POI _asbp_game_instance)) 1)))))))

(fn GetRandomMapStage3
  (params (type :type Integer))
  (bind _asbp_game_instance (Utilities|Casting|CastToBP_GameInstance (Game|GetGameInstance)))
  (switch int type
    (:0
      (return (Utilities|Array|Get(acopy) (Variables|/Game/Core/General/BP_GameInstance.BP_GameInstance_C|GetmapNamesStage3 _asbp_game_instance) (Math|Random|RandomIntegerinRange 0 (- (Utilities|Array|Length (Variables|/Game/Core/General/BP_GameInstance.BP_GameInstance_C|GetmapNamesStage3 _asbp_game_instance)) 1)))))
    (:1
      (return (Utilities|Array|Get(acopy) (Variables|/Game/Core/General/BP_GameInstance.BP_GameInstance_C|GetmapNamesStage3_City _asbp_game_instance) (Math|Random|RandomIntegerinRange 0 (- (Utilities|Array|Length (Variables|/Game/Core/General/BP_GameInstance.BP_GameInstance_C|GetmapNamesStage3_City _asbp_game_instance)) 1)))))
    (:2
      (return (Utilities|Array|Get(acopy) (Variables|/Game/Core/General/BP_GameInstance.BP_GameInstance_C|GetmapNamesStage3_POI _asbp_game_instance) (Math|Random|RandomIntegerinRange 0 (- (Utilities|Array|Length (Variables|/Game/Core/General/BP_GameInstance.BP_GameInstance_C|GetmapNamesStage3_POI _asbp_game_instance)) 1)))))))