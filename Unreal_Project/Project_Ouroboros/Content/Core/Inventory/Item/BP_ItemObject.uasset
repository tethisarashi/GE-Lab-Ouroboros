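; BP_ItemObject is an inventory item data object holding name, ID, type, icons, dimensions, and separate player and merchant prices.
; Rotate toggles the IsRotated flag, which makes GetDimensions swap X and Y and GetIcon return the rotated icon, suggesting a grid-based inventory.
; The remaining functions are simple getters for the stored fields.
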(fn GetDimensions
  (bind _dimensions (Variables|Default|GetDimensions))
  (if (Variables|Private|GetisRotated)
    (return (Utilities|Struct|MakeIntPoint (.y _dimensions) (.x _dimensions)))
    (else
      (return (Variables|Default|GetDimensions)))))

(fn GetIcon
  (return (select (Variables|Private|GetisRotated) (Variables|Default|GetIconRotated) (Variables|Default|GetIcon))))

(fn Rotate
  (Variables|Private|SetisRotated (not (Variables|Private|GetisRotated)))
  (return))

(fn GetIsRotated
  (return (Variables|Private|GetisRotated)))

(fn GetItemType
  (return (Variables|Private|GetitemType)))

(fn GetIconRotated
  (return (Variables|Default|GetIconRotated)))

(fn GetItemName
  (return (Variables|Default|GetitemName)))

(fn GetItemID
  (return (Variables|Private|GetitemID)))

(fn GetItemPlayerPrice
  (return (Variables|Private|GetplayerPrice)))

(fn GetItemMerchantPrice
  (return (Variables|Private|GetmerchantPrice)))